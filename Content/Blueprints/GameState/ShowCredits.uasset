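; ShowCredits is a game state that starts the end credits when created.
; On creation it disables player input, plays the general fade-out level sequence, and starts the credits music through a newly created audio component.
; A timer matched to the sequence length then adds the credit screen widget to the viewport and hides the quest goal.
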(event Custom|CustomEvent_0
  (bind _widget_instance (Default|CreateWidget (Variables|Default|GetGameMode) "/Game/Blueprints/UI/CreditScreenUI.CreditScreenUI_C"))
  (UserInterface|Viewport|AddtoViewport _widget_instance 0)
  (CallFunction|HideQuestGoal))

(event EventCreated
  (bind _gamemode (Variables|Default|GetGameMode))
  (Default|DisablePlayerInput _gamemode)
  (bind _newsequence (Default|CreateLevelSequencePlayer _gamemode "/Game/Animations/Seq_General_FadeOut.Seq_General_FadeOut"))
  (Audio|Components|Audio|Play _newsequence)
  (Utilities|Time|SetTimerbyEvent (delegate Custom|CustomEvent_0) (Class|LevelSequencePlayer|GetLength _newsequence))
  (bind _output_get (Variables|Default|SetAudioComponent (Class|LowEntryExtendedStandardLibrary|CreateObject "/Script/Engine.AudioComponent")))
  (Audio|Components|Audio|SetSound _output_get "/Game/Audio/Sounds/Start_Credit_Level/credits2_Cue.credits2_Cue")
  (Audio|Components|Audio|Play _output_get 0.0))