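; Placeholder game state for the loading screen that completes once the GameMode reports loading is done, polled on Tick.
; When disabled, it clears the Quest 01-01 setup, turning off trigger volume collision and particles.
; For each trigger found, it also hides the sister, father and mother characters, disables their collision and fades out the ambient fighting sound.
; Actors are looked up by class and hardcoded name through the GameMode.
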(event EventTick
  (if (Variables|/Game/Blueprints/GameState/SeriousStressGameMode.SeriousStressGameMode_C|GetLoadingDone (Variables|Default|GetGameMode))
    (Default|CallOnCompleted)))

(event EventDisabled
  (bind _gamemode (Variables|Default|GetGameMode))
  (bind _actorarray (Default|GetActorsbyClass (Variables|Default|GetGameMode) "/Game/Blueprints/InteractiveObjects/Quests/Quest_01-01_triggerVolume.Quest_01-01_triggerVolume_C"))
  (for _array_element _actorarray
    (bind _asquest_01_01_trigger_volume (Utilities|Casting|CastToQuest_01-01_triggerVolume _array_element))
    (Collision|SetCollisionEnabled (Variables|/Game/Blueprints/InteractiveObjects/Quests/Quest_01-01_triggerVolume.Quest_01-01_triggerVolume_C|GetTriggerBox _asquest_01_01_trigger_volume) "NoCollision")
    (Rendering|SetVisibility (Variables|/Game/Blueprints/InteractiveObjects/Quests/Quest_01-01_triggerVolume.Quest_01-01_triggerVolume_C|GetParticleSystem _asquest_01_01_trigger_volume) false false)
    (bind _actor (Default|GetActorbyClassandName _gamemode "/Game/Blueprints/Characters/InteractableCharacter.InteractableCharacter_C" "Quest_01-01_SisterChar"))
    (bind _asinteractable_character (Utilities|Casting|CastToInteractableCharacter _actor))
    (Default|DisableCollision _asinteractable_character)
    (Rendering|SetActorHiddenInGame _asinteractable_character true)
    (bind _actor_2 (Default|GetActorbyClassandName _gamemode "/Game/Blueprints/Characters/InteractableCharacter.InteractableCharacter_C" "FatherChar_Day01-01"))
    (bind _asinteractable_character_2 (Utilities|Casting|CastToInteractableCharacter _actor_2))
    (Default|DisableCollision _asinteractable_character_2)
    (Rendering|SetActorHiddenInGame _asinteractable_character_2 true)
    (bind _actor_3 (Default|GetActorbyClassandName _gamemode "/Game/Blueprints/Characters/InteractableCharacter.InteractableCharacter_C" "MotherChar_Day01-01"))
    (bind _asinteractable_character_3 (Utilities|Casting|CastToInteractableCharacter _actor_3))
    (Default|DisableCollision _asinteractable_character_3)
    (Rendering|SetActorHiddenInGame _asinteractable_character_3 true)
    (CallFunction|StopAmbientDlg)))

(fn StopAmbientDlg
  (bind _actor (Default|GetActorbyName (Variables|Default|GetGameMode) "Quest_01-01_AmbientFighting"))
  (bind _asambient_sound (Utilities|Casting|CastToAmbientSound _actor))
  (Audio|Components|Audio|FadeOut (Variables|/Script/Engine.AmbientSound|GetAudioComponent _asambient_sound) 0.3 0.0 :!class /Script/Engine.AudioComponent))