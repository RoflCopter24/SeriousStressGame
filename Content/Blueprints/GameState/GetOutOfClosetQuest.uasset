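; A quest object for "Task 2", which tells the player to leave the closet.
; On creation it prints its name and description and uses the GameMode to find and cache the ChildRoom_Closet actor by class and name.
; Its per-frame Tick polls that closet and completes the quest once, when the player is no longer inside and the left door is closed.
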(event EventCreated
  (bind _gamemode (Variables|Default|GetGameMode))
  ;[1 1 1] Initialization
  (bind _output_get (Variables|Default|SetName "Task 2"))
  (bind _output_get_2 (Variables|Default|SetDescription "Leave the closet!"))
  (Utilities|IsValid _gamemode
    (:Is%20Valid
      (Development|PrintString _gamemode (Class|VictoryBPFunctionLibrary|AppendMultiple (Utilities|String|ToString(Text) _output_get) ": " (Utilities|String|ToString(Text) _output_get_2)) true true "(R=0.000000,G=0.660000,B=1.000000,A=1.000000)" 8.0)
      (bind _actor (Default|GetActorbyClassandName _gamemode "/Game/Blueprints/InteractiveObjects/ChildRoom_Closet.ChildRoom_Closet_C" "ChildRoom_Closet"))
      (Utilities|IsValid _actor
        (:Is%20Valid
          (bind _aschild_room_closet (Utilities|Casting|CastToChildRoom_Closet _actor))
          (Variables|Default|SetChildRoomCloset _aschild_room_closet))))
    (:Is%20Not%20Valid
      (Development|PrintString _gamemode "Game Mode pointer invalid"))))

(event EventTick
  (bind _childroomcloset (Variables|Default|GetChildRoomCloset))
  ;[1 1 1] Check Quest Objective Condition (called every frame)
  (if (not (Variables|Default|GetbCompleted))
    (Utilities|IsValid _childroomcloset
      (:Is%20Valid
        (if (not (Variables|/Game/Blueprints/InteractiveObjects/ChildRoom_Closet.ChildRoom_Closet_C|GetIsPlayerInside _childroomcloset))
          (if (not (Variables|/Game/Blueprints/InteractiveObjects/ChildRoom_Closet.ChildRoom_Closet_C|GetIsLeftDoorOpen _childroomcloset))
            (Default|CallOnCompleted)
            (Variables|Default|SetbCompleted true))))
      (:Is%20Not%20Valid
        (Development|PrintString (Variables|Default|GetGameMode) "Closet obj not valid")))))