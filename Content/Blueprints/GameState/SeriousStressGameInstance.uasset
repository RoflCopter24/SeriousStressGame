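; Game instance for SeriousStress that switches game states between main menu, settings menu and gameplay, and offers a dynamic resolution scaling helper.
; SetGameState shows menus directly on MenuMap, otherwise clears widgets and loads MenuMap with an option or the Flat level; Init's Intro state has no handling.
; AdjustResScale steps resolution by a twentieth of maximum based on FPS thresholds, but jumps to maximum when a downscale would reach minimum.
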(event EventInit
  (GameState|SetGameState "NewEnumerator0"))

(fn SetGameState
  (params (targetState :type E_SSGState%20Enum))
  (switch Utilities|FlowControl|Switch|SwitchonE_SSGState targetState
    (:NewEnumerator1
      ;[1 1 1] Switch to main menu
      (bind _returnvalue (Game|GetCurrentLevelName true))
      (if (Utilities|Enum|Equal(Enum) _returnvalue "MenuMap")
        (Default|CallOnShowMainMenu)
        (else
          (Viewport|RemoveAllWidgets)
          (Game|OpenLevel(byName) "MenuMap" true "main"))))
    (:NewEnumerator2
      ;[1 1 1] Switch to Settings menu
      (bind _returnvalue_2 (Game|GetCurrentLevelName true))
      (if (Utilities|Enum|Equal(Enum) _returnvalue_2 "MenuMap")
        (Default|CallOnShowSettingsMenu)
        (else
          (Viewport|RemoveAllWidgets)
          (Game|OpenLevel(byName) "MenuMap" true "settings"))))
    (:NewEnumerator3
      ;[1 1 1] Switch to Gameplay
      (bind _returnvalue_3 (Game|GetCurrentLevelName true))
      (if (not (Utilities|Enum|Equal(Enum) _returnvalue_3 "Flat"))
        (Viewport|RemoveAllWidgets)
        (Game|OpenLevel(byName) "Flat")))))

(fn AdjustResScale
  (params (Delta :type Float%20%28single-precision%29) (DownScaleBelow :type Float%20%28single-precision%29) (UpScaleAbove :type Float%20%28single-precision%29))
  (bind _returnvalue (/ 1.0 Delta))
  (if (< _returnvalue DownScaleBelow)
    (bind _returnvalue_2 (Settings|GetGameUserSettings))
    (Utilities|IsValid _returnvalue_2
      (:Is%20Valid
        (if (> (- (.CurrentScaleValue (Class|GameUserSettings|GetResolutionScaleInformationEx _returnvalue_2)) (/ (.MaxScaleValue (Class|GameUserSettings|GetResolutionScaleInformationEx _returnvalue_2)) 2e+01)) (.MinScaleValue (Class|GameUserSettings|GetResolutionScaleInformationEx _returnvalue_2)))
          (Class|GameUserSettings|SetResolutionScaleValueEx _returnvalue_2 (- (.CurrentScaleValue (Class|GameUserSettings|GetResolutionScaleInformationEx _returnvalue_2)) (/ (.MaxScaleValue (Class|GameUserSettings|GetResolutionScaleInformationEx _returnvalue_2)) 2e+01)))
          (else
            (Class|GameUserSettings|SetResolutionScaleValueEx _returnvalue_2 (.MaxScaleValue (Class|GameUserSettings|GetResolutionScaleInformationEx _returnvalue_2))))))
      (:Is%20Not%20Valid
        _))
    (elif (> _returnvalue UpScaleAbove)
      (bind _returnvalue_3 (Settings|GetGameUserSettings))
      (Utilities|IsValid _returnvalue_3
        (:Is%20Valid
          (if (< (+ (.CurrentScaleValue (Class|GameUserSettings|GetResolutionScaleInformationEx _returnvalue_3)) (/ (.MaxScaleValue (Class|GameUserSettings|GetResolutionScaleInformationEx _returnvalue_3)) 2e+01)) (.MaxScaleValue (Class|GameUserSettings|GetResolutionScaleInformationEx _returnvalue_3)))
            (Class|GameUserSettings|SetResolutionScaleValueEx _returnvalue_3 (+ (.CurrentScaleValue (Class|GameUserSettings|GetResolutionScaleInformationEx _returnvalue_3)) (/ (.MaxScaleValue (Class|GameUserSettings|GetResolutionScaleInformationEx _returnvalue_3)) 2e+01)))
            (else
              (Class|GameUserSettings|SetResolutionScaleValueEx _returnvalue_3 (.MaxScaleValue (Class|GameUserSettings|GetResolutionScaleInformationEx _returnvalue_3))))))
        (:Is%20Not%20Valid
          _))))
  (return (.CurrentScaleValue (Class|GameUserSettings|GetResolutionScaleInformationEx _returnvalue_3))))