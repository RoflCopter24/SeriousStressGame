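; GameFlowItem is a game flow step with empty Created, Tick and Disabled hooks and a toolbox of scene-scripting helpers.
; Helpers work through a GameMode reference, finding actors by name or class, or taking direct references.
; They create prioritized dialogues, rewrite interaction texts, toggle interactions, characters, lights and destructibility, and swap materials.
; Others fade the quest goal widget and fetch the player character or start transforms.
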(fn Tick)

(fn Created)

(fn CreateDialogueInstance
  (params (Priority :type Integer))
  (bind _gamemode (Variables|Default|GetGameMode)
    (:then
      (bind _asserious_stress_game_mode (Utilities|Casting|CastToSeriousStressGameMode _gamemode)
        (:then
          (bind _dialogueuiinstance (Default|CreateDialog _asserious_stress_game_mode))
          (Variables|/Game/Blueprints/UI/DialogueUi.DialogueUi_C|SetDialoguePriority _dialogueuiinstance Priority))
        (:CastFailed
          _)))
    (:else
      _))
  (return _dialogueuiinstance))

(fn ChangeDlgInstancesOfClass
  (params (InteractableObject :type Interactable%20Object%20Class%20Reference) (LeftDialogueText :type Text) (RightDialogueText :type Text))
  (bind _gamemode (Variables|Default|GetGameMode)
    (:then
      (bind _actorarray (Default|GetActorsbyClass _gamemode InteractableObject))
      (for _array_element _actorarray
        (bind _asinteractable_object (Utilities|Casting|CastToInteractableObject _array_element))
        (Variables|/Game/Blueprints/InteractiveObjects/InteractableObject.InteractableObject_C|SettextLeftInteractionDialogue _asinteractable_object LeftDialogueText)
        (Variables|/Game/Blueprints/InteractiveObjects/InteractableObject.InteractableObject_C|SettextRightInteractionDialogue _asinteractable_object RightDialogueText))
      (return))
    (:else)))

(fn ChangeDlgInstanceOfActor
  (params (ActorReference :type Actor%20Object%20Reference) (ActorName :type String) (NewLeftInteractionText :type Text) (NewRightInteractionText :type Text))
  (bind _returnvalue (Utilities|GetClass ActorReference))
  (if (Utilities|Enum|NotEqual(Enum) ActorName "")
    ;[1 1 1] By Name
    (bind _actor (Default|GetActorbyName (Variables|Default|GetGameMode) ActorName))
    (Utilities|IsValid _actor
      (:Is%20Valid
        (if (Utilities|ClassIsChildOf (Utilities|GetClass _actor) "/Game/Blueprints/InteractiveObjects/InteractableObject.InteractableObject_C")
          (bind _asinteractable_object (Utilities|Casting|CastToInteractableObject _actor)
            (:then
              (Variables|/Game/Blueprints/InteractiveObjects/InteractableObject.InteractableObject_C|SettextLeftInteractionDialogue _asinteractable_object NewLeftInteractionText)
              (Variables|/Game/Blueprints/InteractiveObjects/InteractableObject.InteractableObject_C|SettextRightInteractionDialogue _asinteractable_object NewRightInteractionText))
            (:CastFailed
              (Development|PrintString _actor "ERROR: Cast failed in ChangeDlgInstanceOfActor by Name" true true "(R=1.000000,G=0.017204,B=0.000000,A=1.000000)" 4.0 :!label _label)))
          (elif (Utilities|ClassIsChildOf (Utilities|GetClass _actor) "/Game/Blueprints/Characters/InteractableCharacter.InteractableCharacter_C")
            (bind _asinteractable_character (Utilities|Casting|CastToInteractableCharacter _actor)
              (:then
                (Variables|/Game/Blueprints/Characters/InteractableCharacter.InteractableCharacter_C|SettextLeftInteraction _asinteractable_character NewLeftInteractionText)
                (Variables|/Game/Blueprints/Characters/InteractableCharacter.InteractableCharacter_C|SettextRightInteraction _asinteractable_character NewRightInteractionText))
              (:CastFailed
                (goto _label)))
            (else
              (Development|PrintString 0 "ERROR: Actor is neither InteractableObject nor InteractableCharacter!" true true "(R=1.000000,G=0.008162,B=0.000000,A=1.000000)" 4.0)))))
      (:Is%20Not%20Valid
        (Development|PrintString 0 "ERROR: GetActorByName failed in ChangeDlgInstanceOfActor! " true true "(R=1.000000,G=0.000000,B=0.016900,A=1.000000)" 4.0)))
    (else
      ;[1 1 1] From Actor Reference
      (Utilities|IsValid ActorReference
        (:Is%20Valid
          (if (Utilities|ClassIsChildOf _returnvalue "/Game/Blueprints/InteractiveObjects/InteractableObject.InteractableObject_C")
            (bind _asinteractable_object_2 (Utilities|Casting|CastToInteractableObject ActorReference)
              (:then
                (Variables|/Game/Blueprints/InteractiveObjects/InteractableObject.InteractableObject_C|SettextLeftInteractionDialogue _asinteractable_object_2 NewLeftInteractionText)
                (Variables|/Game/Blueprints/InteractiveObjects/InteractableObject.InteractableObject_C|SettextRightInteractionDialogue _asinteractable_object_2 NewRightInteractionText))
              (:CastFailed
                (Development|PrintString ActorReference "ERROR: Cast failed in ChangeDlgInstanceOfActor by Ref!" :!label _label_2)))
            (elif (Utilities|ClassIsChildOf _returnvalue "/Game/Blueprints/Characters/InteractableCharacter.InteractableCharacter_C")
              (bind _asinteractable_character_2 (Utilities|Casting|CastToInteractableCharacter ActorReference)
                (:then
                  (Variables|/Game/Blueprints/Characters/InteractableCharacter.InteractableCharacter_C|SettextLeftInteraction _asinteractable_character_2 NewLeftInteractionText)
                  (Variables|/Game/Blueprints/Characters/InteractableCharacter.InteractableCharacter_C|SettextRightInteraction _asinteractable_character_2 NewRightInteractionText))
                (:CastFailed
                  (goto _label_2)))
              (else
                (Development|PrintString ActorReference "ERROR: Actor is neither InteractableObject nor InteractableCharacter!" true true "(R=1.000000,G=0.008162,B=0.000000,A=1.000000)" 4.0)))))
        (:Is%20Not%20Valid
          (Development|PrintString (Variables|Default|GetGameMode) "ERROR: Actor ref invalid in ChangeDlgInstanceOfActor!")))))
  (return))

(fn Disabled)

(fn GetPlayerCharRef
  (bind _player_controller (Default|GetPlayerControllerPub (Variables|Default|GetGameMode)))
  (bind _aschild_first_person_character (Utilities|Casting|CastToChildFirstPersonCharacter (Pawn|GetControlledPawn _player_controller))
    (:then
      _)
    (:CastFailed
      (Development|PrintString 0 "ERROR: Controlled Pawn not of type ChildFirstPersonCharacter! (Seq_Day3_01-DayIntro_BP)" true true "(R=1.000000,G=0.000000,B=0.007639,A=1.000000)")))
  (return _aschild_first_person_character))

(fn IsChildFPChar
  (params (Object :type Actor%20Object%20Reference))
  (return (== (Utilities|GetClass Object) "/Game/Blueprints/Characters/ChildFirstPersonCharacter.ChildFirstPersonCharacter_C")))

(fn HideQuestGoal
  (Default|DoFadeOut (Variables|/Game/Blueprints/GameState/SeriousStressGameMode.SeriousStressGameMode_C|GetQuestGoalWidget (Variables|Default|GetGameMode)) (EventDispatchers|CreateEvent :!event Dummy)))

(fn Dummy)

(fn GetPlayerStart
  (params (Name :type String))
  (bind _actor (Default|GetActorbyClassandName (Variables|Default|GetGameMode) "/Script/Engine.PlayerStart" Name))
  (return (Transformation|GetActorTransform _actor)))

(fn SetPointlightVisibility
  (params (name :type String) (Visible :type Boolean))
  (bind _actor (Default|GetActorbyClassandName (Variables|Default|GetGameMode) "/Script/Engine.PointLight" name))
  (bind _aspoint_light (Utilities|Casting|CastToPointLight _actor)
    (:then
      (Rendering|SetVisibility (Variables|/Script/Engine.PointLight|GetPointLightComponent _aspoint_light) Visible false)
      (Rendering|SetVisibility (Variables|/Script/Engine.Light|GetLightComponent _aspoint_light) Visible false)
      (return))
    (:CastFailed
      (return))))

(fn ShowQuestGoal
  (Default|DoFadein (Variables|/Game/Blueprints/GameState/SeriousStressGameMode.SeriousStressGameMode_C|GetQuestGoalWidget (Variables|Default|GetGameMode)) (EventDispatchers|CreateEvent :!event Dummy))
  (return))

(fn SetInteractableCharacterEnabled
  (params (Enabled :type Boolean) (Target :type Interactable%20Character%20Object%20Reference))
  (if Enabled
    (Default|EnableCollision Target)
    (Rendering|SetVisibility (Variables|/Script/Engine.Character|GetMesh Target) true true)
    (Rendering|ToggleVisibility (Variables|/Script/Engine.Character|GetCapsuleComponent Target) true)
    (Rendering|SetActorHiddenInGame Target false)
    (else
      (Default|DisableCollision Target)
      (Rendering|SetVisibility (Variables|/Script/Engine.Character|GetMesh Target) false true)
      (Rendering|ToggleVisibility (Variables|/Script/Engine.Character|GetCapsuleComponent Target) true)))
  (return))

(fn SetDestructiblesState
  (params (Destructable :type Boolean))
  (bind _actorarray (Default|GetActorsbyClass (Variables|Default|GetGameMode) "/Game/Blueprints/InteractiveObjects/DestructableCaryableObject.DestructableCaryableObject_C"))
  (for _array_element _actorarray
    (bind _asdestructable_caryable_object (Utilities|Casting|CastToDestructableCaryableObject _array_element))
    (Variables|/Game/Blueprints/InteractiveObjects/DestructableCaryableObject.DestructableCaryableObject_C|SetDestructible _asdestructable_caryable_object Destructable))
  (return))

(fn SetActorInteractionEnabled
  (params (Name :type String) (LeftInteraction :type Boolean) (RightInteraction :type Boolean))
  (bind _gamemode (Variables|Default|GetGameMode))
  (bind _actor (Default|GetActorbyClassandName _gamemode "/Game/Blueprints/InteractiveObjects/InteractableObject.InteractableObject_C" Name))
  (bind _asinteractable_object (Utilities|Casting|CastToInteractableObject _actor)
    (:then
      (Variables|/Game/Blueprints/InteractiveObjects/InteractableObject.InteractableObject_C|SetbRightInteraction _asinteractable_object RightInteraction)
      (Variables|/Game/Blueprints/InteractiveObjects/InteractableObject.InteractableObject_C|SetbLeftInteraction _asinteractable_object LeftInteraction))
    (:CastFailed
      (Development|PrintString _gamemode (Class|VictoryBPFunctionLibrary|AppendMultiple "WARNING: Could not find InteractableObject with Name \"" Name "\" in [SetActorInteractionEnabled] of GameFlowItem!") true true "(R=1.000000,G=0.699787,B=0.000000,A=1.000000)" 4.0)))
  (return))

(fn ChangeMaterialforStaticMeshActor
  (params (ThisActor-> :type Actor%20Object%20Reference) (WithThisName-> :type String) (AllOfThisClass%20-> :type Actor%20Class%20Reference) (NewMaterial :type Material%20Object%20Reference))
  (bind _returnvalue (Actor|GetComponentbyClass ThisActor-> "/Script/Engine.StaticMeshComponent"))
  (bind _gamemode (Variables|Default|GetGameMode))
  (Utilities|IsValid ThisActor->
    (:Is%20Valid
      (if (Utilities|IsValid _returnvalue)
        (Rendering|Material|SetMaterial _returnvalue 0 NewMaterial)
        (else
          (Development|PrintString 0 "No valid StaticMeshComponent!" true true "(R=1.000000,G=0.773061,B=0.000000,A=1.000000)" 5.0))))
    (:Is%20Not%20Valid
      (if (> (Utilities|String|Len WithThisName->) 0)
        (bind _actor (Default|GetActorbyName _gamemode WithThisName->))
        (if (Utilities|IsValid (Actor|GetComponentbyClass _actor "/Script/Engine.StaticMeshComponent"))
          (Rendering|Material|SetMaterial (Actor|GetComponentbyClass _actor "/Script/Engine.StaticMeshComponent") 0 NewMaterial))
        (else
          (if (Utilities|IsValidClass AllOfThisClass%20->)
            (bind _actorarray (Default|GetActorsbyClass _gamemode AllOfThisClass%20->))
            (for _array_element _actorarray
              (if (Utilities|IsValid (Actor|GetComponentbyClass _array_element "/Script/Engine.StaticMeshComponent"))
                (Rendering|Material|SetMaterial (Actor|GetComponentbyClass _array_element "/Script/Engine.StaticMeshComponent") 0 NewMaterial))
              (return))
            (else
              (Development|PrintString 0 "[ChangeMaterialForStaticMeshActor] No Parameter gi ven!" true true "(R=1.000000,G=0.838576,B=0.000000,A=1.000000)" 5.0)))
          (return)))))
  (return))