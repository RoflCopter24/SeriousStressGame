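; Game mode that runs the story flow of quests and cutscenes from the Day 1 intro into Day 2.
; GameFlowGraph chains constructed GameFlowItem objects through completion, cancel and fail events, branching on quest 1-03's outcome to set karma before rejoining.
; Only one item is active at a time, and Tick forwards to it.
; It also provides actor lookups, priority-locked dialogue widgets, player input locking and a named player start.
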(event EventBeginPlay)

(event EventTick
  (params (DeltaSeconds :type Float%20%28single-precision%29))
  (for _array_element (Variables|GameFlow|GetGameFlowItems)
    (if (Variables|/Game/Blueprints/GameState/GameFlowItem.GameFlowItem_C|GetbIsActive _array_element)
      (Default|Tick _array_element))))

(event Custom|Quest01_completed
  ;[1 1 1] Quest Day 01 - 01
  ;[1 1 1] Quest Day01-02
  (bind _gameflowiteminstance (GameFlow|CreateGameFlowItem "/Game/Blueprints/GameState/Quests/Quest_01-02.Quest_01-02_C" true))
  (EventDispatchers|BindEventtoOnCompleted _gameflowiteminstance (delegate Custom|QuestDay1-02Complete)))

(event Custom|Day02_01_completed
  ;[1 1 1] QuestDay 02/01
)

(event Custom|Quest_Day01-03_Ending01
  ;[1 1 1] Quest Day 01-03
  ;[1 1 1] Quest Day01 04-1
  (bind _gameflowiteminstance (GameFlow|CreateGameFlowItem "/Game/Blueprints/Cutscenes/Seq_Day1_04-1_ToysInChest_BP.Seq_Day1_04-1_ToysInChest_BP_C" true))
  (EventDispatchers|BindEventtoOnCompleted _gameflowiteminstance (delegate Custom|Quest_Day01-04-1_finished)))

(event Custom|Quest01_Canceled
  ;[1 1 1] Quest Day 01 - 01
  ;[1 1 1] Quest Day01-02
  (bind _gameflowiteminstance (GameFlow|CreateGameFlowItem "/Game/Blueprints/GameState/Quests/Quest_01-02.Quest_01-02_C" true))
  (EventDispatchers|BindEventtoOnCompleted _gameflowiteminstance (delegate Custom|QuestDay1-02Complete)))

(event Custom|Quest_Day01-03_Ending02
  ;[1 1 1] Quest Day 01-03
  ;[1 1 1] Quest Day01 04-2
  (bind _gameflowiteminstance (GameFlow|CreateGameFlowItem "/Game/Blueprints/Cutscenes/Seq_Day1_04-1_ToysInChest_BP.Seq_Day1_04-1_ToysInChest_BP_C" true))
  (EventDispatchers|BindEventtoOnCompleted _gameflowiteminstance (delegate Custom|Quest_Day01-04-2_finished)))

(event Custom|Active%20GameFlowItem%20changed
  (params (NewGameFlowItem :type Game%20Flow%20Item%20Object%20Reference))
  ;[1 1 1] Active Quest changed
  (Development|PrintString (Class|VictoryBPFunctionLibrary|StringCombineStringsMulti "Active GameFlow Item changed to: " (Utilities|GetDisplayName NewGameFlowItem)) true true "(R=1.000000,G=1.000000,B=1.000000,A=1.000000)" 5.0))

(event Custom|CutSceneDay01Intro_Finished
  ;[1 1 1] Intro Day 1
  ;[1 1 1] Quest Day 01 - 01
  (bind _gameflowiteminstance (GameFlow|CreateGameFlowItem "/Game/Blueprints/GameState/Quests/Quest_01-01.Quest_01-01_C" true))
  (EventDispatchers|AssignOnCompleted _gameflowiteminstance (delegate Custom|Quest01_completed))
  (EventDispatchers|BindEventtoOnCanceled _gameflowiteminstance (delegate Custom|Quest01_Canceled)))

(event Custom|QuestDay1-02Complete
  ;[1 1 1] Quest Day01-02
  ;[1 1 1] Quest Day 01-03
  (bind _gameflowiteminstance (GameFlow|CreateGameFlowItem "/Game/Blueprints/GameState/Quests/Quest_01-03.Quest_01-03_C" true))
  (EventDispatchers|BindEventtoOnCompleted _gameflowiteminstance (delegate Custom|Quest_Day01-03_Ending01))
  (EventDispatchers|BindEventtoOnFailed _gameflowiteminstance (delegate Custom|Quest_Day01-03_Ending02)))

(event Custom|Quest_Day01-04-1_finished
  ;[1 1 1] Quest Day01 04-1
  (Game|AddKarma 1)
  ;[1 1 1] QuestDay 02/01
  (bind _gameflowiteminstance (GameFlow|CreateGameFlowItem "/Game/Blueprints/GameState/Quests/Quest_02-01.Quest_02-01_C" true))
  (EventDispatchers|BindEventtoOnCompleted _gameflowiteminstance (delegate Custom|Day02_01_completed)))

(event Custom|CutSceneDay01Intro_Canceled
  ;[1 1 1] Intro Day 1
  ;[1 1 1] Quest Day 01 - 01
  (bind _gameflowiteminstance (GameFlow|CreateGameFlowItem "/Game/Blueprints/GameState/Quests/Quest_01-01.Quest_01-01_C" true))
  (EventDispatchers|AssignOnCompleted _gameflowiteminstance (delegate Custom|Quest01_completed))
  (EventDispatchers|BindEventtoOnCanceled _gameflowiteminstance (delegate Custom|Quest01_Canceled)))

(event Custom|Quest_Day01-04-2_finished
  ;[1 1 1] Quest Day01 04-2
  (Game|AddKarma)
  ;[1 1 1] QuestDay 02/01
  (bind _gameflowiteminstance (GameFlow|CreateGameFlowItem "/Game/Blueprints/GameState/Quests/Quest_02-01.Quest_02-01_C" true))
  (EventDispatchers|BindEventtoOnCompleted _gameflowiteminstance (delegate Custom|Day02_01_completed)))

(event EventBeginPlay
  ;[1 1 1] Intro Day 1
  (bind _gameflowiteminstance (GameFlow|CreateGameFlowItem "/Game/Blueprints/Cutscenes/Seq_Day1_01Intro_BP.Seq_Day1_01Intro_BP_C" true))
  (EventDispatchers|BindEventtoOnCompleted _gameflowiteminstance (delegate Custom|CutSceneDay01Intro_Finished))
  (EventDispatchers|BindEventtoOnCanceled _gameflowiteminstance (delegate Custom|CutSceneDay01Intro_Canceled)))

(fn ConstructionScript
  (|CallParentFunction)
  (Game|ResetKarmaCount))

(fn AddKarma
  (params (Karma :type Integer))
  (if (>= Karma 0)
    (bind _output_get (Variables|Game|SetkarmaCounter Karma))
    (Development|PrintString (Utilities|String|BuildString(Integer) "Karma is now set to: " "" _output_get) true true "(R=0.130561,G=1.000000,B=0.000000,A=1.000000)")
    (else
      (Development|PrintText "WARNING: Tried to set negative Karma value" true true "(R=1.000000,G=0.465393,B=0.000000,A=1.000000)" 3.0))))

(fn GetKarmaCount
  (return (Variables|Game|GetkarmaCounter)))

(fn ResetKarmaCount
  (Variables|Game|SetkarmaCounter 0)
  (Development|PrintString "Karma reser to 0" true true "(R=1.000000,G=0.000000,B=0.702293,A=1.000000)"))

(fn CreateGameFlowItem
  (params (GameFlowItemClass :type Game%20Flow%20Item%20Class%20Reference) (SetActive :type Boolean))
  (bind _self self)
  (bind _returnvalue (Game|ConstructObjectfromClass GameFlowItemClass _self))
  (bind _output_get (LocalVariables|SetItemInstance _returnvalue))
  (Variables|/Game/Blueprints/GameState/GameFlowItem.GameFlowItem_C|SetGameMode _output_get _self)
  (GameFlow|SetGameFlowItemActive _output_get)
  (Utilities|Array|Add (Variables|GameFlow|GetGameFlowItems) _output_get)
  (Default|Created _output_get)
  (return _output_get))

(fn SetGameFlowItemActive
  (params (Item :type Game%20Flow%20Item%20Object%20Reference))
  (for _array_element (Variables|GameFlow|GetGameFlowItems)
    (if (Variables|/Game/Blueprints/GameState/GameFlowItem.GameFlowItem_C|GetbIsActive _array_element)
      (Variables|/Game/Blueprints/GameState/GameFlowItem.GameFlowItem_C|SetbIsActive _array_element false)))
  (Variables|/Game/Blueprints/GameState/GameFlowItem.GameFlowItem_C|SetbIsActive Item true)
  (CallFunction|ActiveGameFlowItemChanged Item))

(fn GetActorbyName
  (params (Name :type String))
  (bind _outactors (Actor|GetAllActorsOfClass "/Script/Engine.Actor"))
  (bind _array_element (Utilities|ReversedforEachLoop _outactors)
    (:LoopBody
      (if (Utilities|Enum|Equal(Enum) (Utilities|GetObjectName _array_element) Name)
        (LocalVariables|SetOutResult _array_element)))
    (:Completed
      (return (LocalVariables|GetOutResult)))))

(fn GetActorsbyClass
  (params (ActorClass :type Actor%20Class%20Reference))
  (bind _outactors (Actor|GetAllActorsOfClass ActorClass))
  (return _outactors))

(fn GetActorbyClassandName
  (params (ActorClass :type Actor%20Class%20Reference) (ActorName :type String))
  (bind _outactors (Actor|GetAllActorsOfClass ActorClass))
  (for _array_element _outactors
    (if (Utilities|Enum|Equal(Enum) (Utilities|GetDisplayName _array_element) ActorName)
      (LocalVariables|SetOutActor _array_element)))
  (return (LocalVariables|GetOutActor)))

(fn GetPlayerControllerPub
  (params (Index :type Integer))
  (return (Game|GetPlayerController Index)))

(fn CreateWidget
  (params (Widget%20Class :type User%20Widget%20Class%20Reference))
  (bind _returnvalue (UserInterface|CreateWidget Widget%20Class (Game|GetPlayerController 0)))
  (return _returnvalue))

(fn CreateDialog
  (bind _widget_instance (Helper|CreateWidget "/Game/Blueprints/UI/DialogueUi.DialogueUi_C"))
  (UserInterface|Viewport|AddtoViewport _widget_instance 0)
  (bind _asdialogue_ui (Utilities|Casting|CastToDialogueUi _widget_instance)
    (:then
      (Variables|/Game/Blueprints/UI/DialogueUi.DialogueUi_C|SetGameMode _asdialogue_ui self))
    (:CastFailed
      _))
  (return _asdialogue_ui))

(fn RequestDialogueLock
  (params (DialogueUiInstance :type Dialogue%20Ui%20Object%20Reference))
  (bind _currentdialogue (Variables|Default|GetCurrentDialogue)
    (:then
      (bind _output_get (LocalVariables|Set_granted (> (Variables|/Game/Blueprints/UI/DialogueUi.DialogueUi_C|GetDialoguePriority DialogueUiInstance) (Variables|/Game/Blueprints/UI/DialogueUi.DialogueUi_C|GetDialoguePriority _currentdialogue))))
      (if _output_get
        (Default|Stop (Variables|Default|GetCurrentDialogue))
        (Widget|RemovefromParent (Variables|Default|GetCurrentDialogue))
        (Variables|Default|SetCurrentDialogue DialogueUiInstance :!label _label)
        (return (LocalVariables|Get_granted))))
    (:else
      (LocalVariables|Set_granted true)
      (goto _label))))

(fn FindPlayerStart
  (params (Player :type Controller%20Object%20Reference) (IncomingName :type String))
  (bind _actor (GameFlow|GetActorbyName "PlayerStartBeginning"))
  (return _actor))

(fn DisablePlayerInputandLookatActor
  (params (ActorName :type String))
  (bind _actor (GameFlow|GetActorbyName ActorName))
  (bind _player_controller (Helper|GetPlayerControllerPub))
  (Input|SetIgnoreLookInput _player_controller true)
  (Input|SetIgnoreMoveInput _player_controller true)
  (Pawn|SetControlRotation _player_controller (Math|Rotator|FindLookatRotation (Transformation|GetActorLocation (Pawn|GetControlledPawn _player_controller)) (Transformation|GetActorLocation _actor)))
  (return false))

(fn EnablePlayerInput
  (bind _player_controller (Helper|GetPlayerControllerPub))
  (Input|SetIgnoreLookInput _player_controller false)
  (Input|SetIgnoreMoveInput _player_controller false))