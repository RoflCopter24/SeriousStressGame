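; Destructible melon actor that stays frozen until its destruction lock is released from outside this graph.
; BeginPlay stores the initial position and sets the lock.
; Every tick, the lock switches physics simulation on the Destructible component off or on, with hard sleeping enabled either way.
; While unlocked, an ApplyDamage value at or above a small threshold is applied every tick as damage with zero-vector hit location and direction.
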(event EventBeginPlay
  (Variables|Default|SetInitialPosition (Transformation|GetActorLocation self))
  (Variables|Default|SetDestructionLocked true))

(event Collision|EventActorBeginOverlap
  (params (OtherActor :type Actor%20Object%20Reference)))

(event EventTick
  (params (DeltaSeconds :type Float%20%28single-precision%29))
  (bind _destructible (Variables|Default|GetDestructible))
  (bind _applydamage (Variables|Melone_destructible|GetApplyDamage))
  (if (Variables|Default|GetDestructionLocked)
    (Variables|/Script/Engine.DestructibleComponent|SetbEnableHardSleeping _destructible true)
    (Physics|SetSimulatePhysics _destructible false)
    (else
      (Variables|/Script/Engine.DestructibleComponent|SetbEnableHardSleeping _destructible true)
      (Physics|SetSimulatePhysics _destructible true)
      (if (>= _applydamage 0.1)
        (Game|Damage|ApplyDamage (Variables|Default|GetDestructible) _applydamage (Math|Vector|MakeVector 0.0 0.0 0.0) (Math|Vector|MakeVector 0.0 0.0 0.0) 0.1)))))

(fn ConstructionScript)