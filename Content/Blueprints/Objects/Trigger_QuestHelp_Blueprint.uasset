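; Trigger actor that shows a one-time quest help screen when the first-person player character enters it.
; It creates the Help widget at BeginPlay and adds it to the player screen on overlap with ChildFirstPersonCharacter.
; Pressing the ShowQuestGoal input removes the widget and sets a flag so later overlaps do not show it again.
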(event EventBeginPlay
  (bind _returnvalue (UserInterface|CreateWidget "/Game/Blueprints/UI/Help.Help_C" (Game|GetPlayerController 0)))
  (Variables|Default|SetHelpWidget _returnvalue))

(event Collision|EventActorBeginOverlap
  (params (OtherActor :type Actor%20Object%20Reference))
  (if (Math|Boolean|ANDBoolean (== (Utilities|GetClass OtherActor) "/Game/Blueprints/Characters/ChildFirstPersonCharacter.ChildFirstPersonCharacter_C") (not (Variables|Default|GetIsDisplayed)) (not (Variables|Default|GetDisplayedOnce)))
    (UserInterface|Viewport|AddtoPlayerScreen (Variables|Default|GetHelpWidget))
    (Variables|Default|SetIsDisplayed true)))

(event EventTick
  (params (DeltaSeconds :type Float%20%28single-precision%29)))

(event Input|ActionEvents|InputActionShowQuestGoal
  (params (Key :type Key%20Structure :default "AnyKey"))
  (:Pressed
    (if (Variables|Default|GetIsDisplayed)
      (Widget|RemovefromParent (Variables|Default|GetHelpWidget))
      (Variables|Default|SetIsDisplayed false)
      (Variables|Default|SetDisplayedOnce true))))

(fn ConstructionScript)