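; Haengeschrank is an interactive wall cabinet with a door that the player can open and close.
; When the left choice is chosen, it flips the IsOpen flag and snaps the Tuer (door) component between closed and a 90-degree open rotation, without animation.
; BeginPlay and the construction script only call their parent versions, and Tick is disabled.
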(event EventBeginPlay
  (|CallParentFunction))

(event Collision|EventActorBeginOverlap
  (params (OtherActor :type Actor%20Object%20Reference)))

(event EventOnLeftChoiceChosen
  (bind _tuer (Variables|Default|GetTuer))
  (if (Variables|Default|GetIsOpen)
    (Transformation|SetRelativeRotation _tuer "0.000000, 0,0.000000" false false)
    (Variables|Default|SetIsOpen false)
    (else
      (Transformation|SetRelativeRotation _tuer "90.000000, 0,0.000000" false false)
      (Variables|Default|SetIsOpen true))))

(event EventTick
  (params (DeltaSeconds :type Float%20%28single-precision%29))
  (|CallParentFunction 0.0))

(fn ConstructionScript
  (|CallParentFunction))