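; DatStuhl is an interactive physics object, apparently a chair by its name, that the first-person player can pick up and drop.
; Pickup flags it as attached and uses a physics constraint to bind its mesh to the player's capsule.
; Drop clears the flag, breaks the constraint and moves its reference position to the mesh's location.
; Carrying is empty, and GetDistanceToPlayer returns the offset vector from player to object.
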(event EventBeginPlay
  (|CallParentFunction))

(event Collision|EventActorBeginOverlap
  (params (OtherActor :type Actor%20Object%20Reference)))

(event EventPickup
  (Variables|Default|SetAttachedToCharacter true)
  (Class|PhysicsConstraintComponent|SetConstrainedComponents (Variables|Default|GetPhysicsConstraint) (Variables|/Script/Engine.Character|GetCapsuleComponent (Variables|Default|GetFpsController)) "None" (Variables|Default|GetObjectMesh) "None"))

(event EventCarrying)

(event EventDrop
  (bind _physicsconstraint (Variables|Default|GetPhysicsConstraint))
  (Variables|Default|SetAttachedToCharacter false)
  (Class|PhysicsConstraintComponent|BreakConstraint _physicsconstraint)
  (Class|PhysicsConstraintComponent|SetConstraintReferencePosition _physicsconstraint "Frame1" (Transformation|GetWorldLocation (Variables|Default|GetObjectMesh))))

(event EventTick
  (params (DeltaSeconds :type Float%20%28single-precision%29))
  (|CallParentFunction 0.0))

(fn ConstructionScript
  (|CallParentFunction))

(fn GetDistancetoPlayer
  (return (- (Transformation|GetActorLocation) (Transformation|GetActorLocation (Variables|Default|GetFpsController)))))