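; An interactive drawer for a flat display case (Schublade flache Vitrine) that opens and closes when the left interaction choice is chosen.
; The choice toggles IsOpen and snaps ObjectMesh between closed and slightly slid-out relative positions, without animation.
; PlaySound restarts the audio component's cue with an Open boolean parameter to distinguish the two actions.
; Opening sets the prompt to "Schließen" (close), but closing never resets it.
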(event EventBeginPlay
  (|CallParentFunction))

(event Collision|EventActorBeginOverlap
  (params (OtherActor :type Actor%20Object%20Reference)))

(event EventTick
  (params (DeltaSeconds :type Float%20%28single-precision%29))
  (|CallParentFunction 0.0))

(event EventOnLeftChoiceChosen
  (bind _objectmesh (Variables|Default|GetObjectMesh))
  (if (Variables|Default|GetIsOpen)
    (CallFunction|PlaySound false)
    (Transformation|SetRelativeLocation _objectmesh "0, 0,0.000000" false false)
    (Variables|Default|SetIsOpen false)
    (else
      (CallFunction|PlaySound true)
      (Transformation|SetRelativeLocation _objectmesh "0,4.000000,0.000000" false false)
      (Variables|Default|SetIsOpen true)
      (Variables|Default|SettextLeftInteraction "Schließen"))))

(fn ConstructionScript
  (|CallParentFunction))

(fn PlaySound
  (params (Open :type Boolean))
  (bind _audio (Variables|Default|GetAudio))
  (Audio|Components|Audio|SetSound _audio (Variables|Default|GetSoundCue))
  (Effects|Components|ParticleSystem|SetBoolParameter _audio "Open" Open)
  (Audio|Components|Audio|Play _audio 0.0))