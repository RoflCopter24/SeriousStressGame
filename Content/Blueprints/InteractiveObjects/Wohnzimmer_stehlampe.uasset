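; Interactive living-room floor lamp whose left dialogue choice switches its lights on or off.
; Choosing it shows the left dialogue, then toggles the visibility of four point lights.
; A LightSwitch boolean is flipped to track the state, though both branches perform the same visibility toggle.
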(event EventBeginPlay
  (|CallParentFunction))

(event Collision|EventActorBeginOverlap
  (params (OtherActor :type Actor%20Object%20Reference)))

(event EventTick
  (params (DeltaSeconds :type Float%20%28single-precision%29))
  (|CallParentFunction 0.0))

(event EventOnLeftChoiceChosen
  (bind _pointlight (Variables|Default|GetPointLight))
  (CallFunction|ShowLeftDialogue)
  (if (Variables|Default|GetLightSwitch)
    (Rendering|ToggleVisibility _pointlight false)
    (Variables|Default|SetLightSwitch false)
    (else
      (Rendering|ToggleVisibility _pointlight false)
      (Variables|Default|SetLightSwitch true))))

(fn ConstructionScript
  (|CallParentFunction))