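; Small kitchen cabinet drawer, an interactive object that opens and closes when its left choice is chosen.
; The choice event checks and flips the IsOpen flag, snapping the object mesh between its closed origin and a slight offset along relative Y, without animation or sweep.
; BeginPlay, overlap and Tick are unused, and the construction script only calls its parent.
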(event EventBeginPlay
  (|CallParentFunction))

(event Collision|EventActorBeginOverlap
  (params (OtherActor :type Actor%20Object%20Reference)))

(event EventTick
  (params (DeltaSeconds :type Float%20%28single-precision%29))
  (|CallParentFunction 0.0))

(event EventOnLeftChoiceChosen
  (bind _objectmesh (Variables|Default|GetObjectMesh))
  (if (Variables|Default|GetIsOpen)
    (Transformation|SetRelativeLocation _objectmesh "0, 0,0.000000" false false)
    (Variables|Default|SetIsOpen false)
    (else
      (Transformation|SetRelativeLocation _objectmesh "0,4.000000,0.000000" false false)
      (Variables|Default|SetIsOpen true))))

(fn ConstructionScript
  (|CallParentFunction))