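; Interactive toy that the player can destroy when its Destructable flag is set, afterwards blocking pickup and offering regretful German dialogue.
; Tick watches the flag through paired DoOnce gates, swapping static and destructible meshes with their physics and toggling the "Zerstören" left interaction.
; Destruct damages the destructible mesh once, using an impulse vector pointing from the toy toward the player camera.
; Physics enable and disable events act on whichever mesh is active.
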(event Custom|Destroy
  (CallFunction|Destruct)
  (Variables|Default|SettextRightInteractionDialogue "Ich hätte es nicht kaputt machen sollen. Aber ich war so wütend!")
  (Variables|Default|SetbLeftInteraction false)
  (Variables|Default|SetPickupBlocked true))

(event EventBeginPlay
  (|CallParentFunction)
  (CallFunction|ToggleDestructiblePhysics false)
  (CallFunction|ToggleStaticMeshPhysics true))

(event Collision|EventActorBeginOverlap
  (params (OtherActor :type Actor%20Object%20Reference)))

(event EventDisablePhysics
  (if (Variables|Default|GetDestructable)
    (CallFunction|ToggleDestructiblePhysics false)
    (else
      (CallFunction|ToggleStaticMeshPhysics false))))

(event EventEnablePhysics
  (if (Variables|Default|GetDestructable)
    (CallFunction|ToggleDestructiblePhysics true)
    (else
      (CallFunction|ToggleStaticMeshPhysics true))))

(event EventTick
  (params (DeltaSeconds :type Float%20%28single-precision%29))
  (|CallParentFunction DeltaSeconds)
  (if (Variables|Default|GetDestructable)
    (Utilities|FlowControl|Sequence
      (:then_0
        (Utilities|FlowControl|DoOnce false :!label _label
          (:Completed
            (CallFunction|SetStaticMeshVisibility false)
            (CallFunction|SetDestructibleVisibility true)
            (Variables|Default|SetbLeftInteraction true)
            (Variables|Default|SettextLeftInteraction "Zerstören")
            (EventDispatchers|BindEventtoOnLeftInteractionChosen (delegate Custom|Destroy)))))
      (:then_1
        (goto _label_2 Reset)))
    (else
      (Utilities|FlowControl|Sequence
        (:then_0
          (Utilities|FlowControl|DoOnce true :!label _label_2
            (:Completed
              (CallFunction|SetDestructibleVisibility false)
              (CallFunction|SetStaticMeshVisibility true)
              (Variables|Default|SetbLeftInteraction false)
              (EventDispatchers|UnbindEventfromOnLeftInteractionChosen (delegate Custom|Destroy)))))
        (:then_1
          (goto _label Reset))))))

(event EventOnRightChoiceChosen
  (if (Variables|Default|GetDestroyed)
    (CallFunction|ShowRightDialogue)
    (else
      (|CallParentFunction))))

(fn ConstructionScript
  (|CallParentFunction))

(fn ToggleDestructiblePhysics
  (params (Active? :type Boolean))
  (bind _destructible (Variables|Default|GetDestructible))
  (bind _destructible_2 (Variables|Default|GetDestructible))
  (Physics|SetEnableGravity (Variables|Default|GetDestructible) Active?)
  (if Active?
    (Collision|SetCollisionEnabled _destructible_2 "QueryAndPhysics")
    (Physics|SetSimulatePhysics _destructible true)
    (else
      (Collision|SetCollisionEnabled _destructible_2 "NoCollision")
      (Physics|SetSimulatePhysics _destructible false)))
  (return))

(fn ToggleStaticMeshPhysics
  (params (Active? :type Boolean))
  (bind _objectmesh (Variables|Default|GetObjectMesh))
  (bind _objectmesh_2 (Variables|Default|GetObjectMesh))
  (Physics|SetEnableGravity _objectmesh Active?)
  (if Active?
    (Collision|SetCollisionEnabled _objectmesh "QueryAndPhysics")
    (Physics|SetSimulatePhysics _objectmesh_2 true)
    (else
      (Collision|SetCollisionEnabled _objectmesh "NoCollision")
      (Physics|SetSimulatePhysics _objectmesh_2 false)))
  (return))

(fn Destruct
  (bind _destructible (Variables|Default|GetDestructible))
  (if (Variables|Default|GetDestructable)
    (if (Variables|Default|GetDestroyed)
      (return)
      (else
        (bind _returnvalue (CallFunction|ComputeImpulseDirection))
        (Game|Damage|ApplyDamage _destructible (Variables|Default|GetDamageApplied) (Transformation|GetWorldLocation _destructible) _returnvalue (Variables|Default|GetDamageStrength))
        (Variables|Default|SetDestroyed true)
        (Development|PrintString "destruct!")
        (return)))
    (else
      (return))))

(fn SetDestructibleVisibility
  (params (Visible :type Boolean))
  (Rendering|SetVisibility (Variables|Default|GetDestructible) Visible true)
  (CallFunction|ToggleDestructiblePhysics Visible))

(fn SetStaticMeshVisibility
  (params (Visible :type Boolean))
  (Rendering|SetVisibility (Variables|Default|GetObjectMesh) Visible true)
  (CallFunction|ToggleStaticMeshPhysics Visible))

(fn ComputeImpulseDirection
  (bind _aschild_first_person_character (Utilities|Casting|CastToChildFirstPersonCharacter (Game|GetPlayerCharacter 0))
    (:then
      (bind _desiredview (Class|CameraComponent|GetCameraView (Variables|/Game/3rdParty/FirstPersonBP/Blueprints/FirstPersonCharacter.FirstPersonCharacter_C|GetFirstPersonCamera _aschild_first_person_character) 0.0)))
    (:CastFailed
      _))
  (return (- (.Location (Utilities|Struct|BreakMinimalViewInfo _desiredview)) (Transformation|GetWorldLocation (Variables|Default|GetDestructible)))))