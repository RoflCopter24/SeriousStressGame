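; Base interactable actor that shows a two-option (left/right) interaction widget while the player aims at it.
; BeginPlay binds events to the widget's option clicks, and Tick toggles visibility from the AimedAt flag.
; Showing the widget enables the options flagged as available and sets their labels.
; The choice handlers are empty stubs, and separate helpers start left or right dialogue through SeriousStressGameMode.
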(event EventBeginPlay
  ;[1 1 1] Register UI Events
  (bind _asinteraction_ui (Utilities|Casting|CastToInteractionUI (UserInterface|GetUserWidgetObject (Variables|Default|GetInteractionWidget)))
    (:then
      (bind _output_get (Variables|Default|SetInteractionUiInstance _asinteraction_ui))
      (EventDispatchers|BindEventtoOnOptionLeftClicked _output_get (EventDispatchers|CreateEvent :!event OnLeftChoiceChosen))
      (EventDispatchers|BindEventtoOnOptionRightClicked _output_get (EventDispatchers|CreateEvent :!event OnRightChoiceChosen)))
    (:CastFailed
      (Development|PrintString "Cast failed"))))

(event Collision|EventActorBeginOverlap
  (params (OtherActor :type Actor%20Object%20Reference)))

(event EventTick
  (params (DeltaSeconds :type Float%20%28single-precision%29))
  (bind _interactionwidget (Variables|Default|GetInteractionWidget))
  (bind _bvisible (Variables|/Script/Engine.SceneComponent|GetbVisible _interactionwidget))
  ;[1 1 1] Determine and set UI visibility
  (if (Variables|Default|GetAimedAt)
    (if (not _bvisible)
      (CallFunction|ShowInteractionUI))
    (elif _bvisible
      (CallFunction|HideInteractionUI))))

(fn ConstructionScript)

(fn ShowInteractionUI
  (bind _interactionwidget (Variables|Default|GetInteractionWidget))
  (bind _returnvalue (UserInterface|GetUserWidgetObject _interactionwidget))
  (Rendering|SetVisibility _interactionwidget true false)
  (Widget|SetVisibility _returnvalue "Visible")
  (bind _asinteraction_ui (Utilities|Casting|CastToInteractionUI _returnvalue))
  (if (Variables|Default|GetbLeftInteraction)
    (Default|EnableOptionLeft _asinteraction_ui))
  (if (Variables|Default|GetbRightInteraction)
    (Default|EnableOptionRight _asinteraction_ui))
  (Default|SetTextLeftOption _asinteraction_ui (Variables|Default|GettextLeftInteraction))
  (Default|SetTextRightOption _asinteraction_ui (Variables|Default|GettextRightInteraction)))

(fn OnLeftChoiceChosen)

(fn OnRightChoiceChosen)

(fn HideInteractionUI
  (bind _interactionwidget (Variables|Default|GetInteractionWidget))
  (Rendering|SetVisibility _interactionwidget false false)
  (Widget|SetVisibility (UserInterface|GetUserWidgetObject _interactionwidget) "Hidden"))

(fn ShowLeftDialogue
  (bind _asserious_stress_game_mode (Utilities|Casting|CastToSeriousStressGameMode (Game|GetGameMode)))
  (bind _dialogueuiinstance (Default|CreateDialog _asserious_stress_game_mode))
  (Default|AddData _dialogueuiinstance 0 (Variables|Default|GettextLeftInteractionDialogue) 0.0)
  (Default|Start _dialogueuiinstance))

(fn ShowRightDialogue
  (bind _asserious_stress_game_mode (Utilities|Casting|CastToSeriousStressGameMode (Game|GetGameMode)))
  (bind _dialogueuiinstance (Default|CreateDialog _asserious_stress_game_mode))
  (Default|AddData _dialogueuiinstance 0 (Variables|Default|GettextRightInteractionDialogue) 0.0)
  (Default|Start _dialogueuiinstance))