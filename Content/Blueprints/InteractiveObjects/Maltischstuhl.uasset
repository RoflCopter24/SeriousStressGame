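; Maltischstuhl is an interactive chair object that responds to left and right choice events.
; The right choice toggles its Standing flag and snaps ObjectMesh between two fixed relative rotations, with no interpolation.
; The left choice calls PlayCameraAnim, which is an empty function in this Blueprint.
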(event EventBeginPlay
  (|CallParentFunction))

(event Collision|EventActorBeginOverlap
  (params (OtherActor :type Actor%20Object%20Reference)))

(event EventOnRightChoiceChosen
  (bind _objectmesh (Variables|Default|GetObjectMesh))
  ;[1 1 1] right choice
  (if (Variables|Default|Getstanding)
    (Transformation|SetRelativeRotation _objectmesh "0, 0,90.000000" false false)
    (Variables|Default|Setstanding false)
    (else
      (Transformation|SetRelativeRotation _objectmesh "85.000000,0.000000,90.000000" false false)
      (Variables|Default|Setstanding true))))

(event EventTick
  (params (DeltaSeconds :type Float%20%28single-precision%29))
  (|CallParentFunction 0.0))

(event EventOnLeftChoiceChosen
  (CallFunction|PlayCameraAnim))

(fn ConstructionScript
  (|CallParentFunction))

(fn PlayCameraAnim)