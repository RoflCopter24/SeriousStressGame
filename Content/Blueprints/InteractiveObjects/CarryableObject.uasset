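; Carryable physics object that the player picks up by holding the Hold input while aiming at it and drops on release.
; Pressing disables mesh physics and attaches the actor to the ChildFirstPersonCharacter cached on BeginPlay; releasing detaches it and restores physics.
; Tick snaps the carried mesh to the character's ObjectAttachment location and turns the interaction widget toward the first-person camera while the object is aimed at.
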(event EventBeginPlay
  (|CallParentFunction)
  (bind _aschild_first_person_character (Utilities|Casting|CastToChildFirstPersonCharacter (Game|GetPlayerCharacter 0)))
  (Variables|Default|SetFpsController _aschild_first_person_character))

(event Collision|EventActorBeginOverlap
  (params (OtherActor :type Actor%20Object%20Reference)))

(event EventTick
  (params (DeltaSeconds :type Float%20%28single-precision%29))
  ;[1 1 1] Rotate UI towards camera
  (|CallParentFunction 0.0)
  (if (Variables|Default|GetAimedAt)
    (Transformation|SetWorldRotation (Variables|Default|GetInteractionWidget) (Math|Rotator|FindLookatRotation (Transformation|GetWorldLocation (Variables|Default|GetObjectMesh)) (.location (Transformation|GetWorldTransform (Variables|/Game/3rdParty/FirstPersonBP/Blueprints/FirstPersonCharacter.FirstPersonCharacter_C|GetFirstPersonCamera (Variables|Default|GetFpsController))))) false false))
  (if (Variables|Default|GetAttachedToCharacter)
    (Transformation|SetWorldLocation (Variables|Default|GetObjectMesh) (Transformation|GetWorldLocation (Variables|/Game/Blueprints/Characters/ChildFirstPersonCharacter.ChildFirstPersonCharacter_C|GetObjectAttachment (Variables|Default|GetFpsController))) false false)))

(event Input|ActionEvents|InputActionHold
  (params (Key :type Key%20Structure :default "AnyKey"))
  ;[1 1 1] Hold object
  (:Pressed
    (Development|PrintString "Pickup!")
    (if (Variables|Default|GetAimedAt)
      (Physics|SetSimulatePhysics (Variables|Default|GetObjectMesh) false)
      (Transformation|AttachActorToActor (Variables|Default|GetFpsController) "None" "SnapToTarget" "SnapToTarget" "KeepRelative" true)
      (Variables|Default|SetAttachedToCharacter true)
      (Development|PrintString "Attached!")))
  (:Released
    (if (Variables|Default|GetAttachedToCharacter)
      (Transformation|DetachFromActor "KeepRelative" "KeepRelative" "KeepRelative")
      (Variables|Default|SetAttachedToCharacter false)
      (Physics|SetSimulatePhysics (Variables|Default|GetObjectMesh) true)
      (Development|PrintString "detached!"))))

(fn ConstructionScript
  (|CallParentFunction))