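; Nachtlicht is an interactive night light Blueprint with a point light that starts deactivated.
; BeginPlay calls the parent logic and deactivates the light, and Tick then mirrors the light's active state onto its visibility every frame.
; Nothing in this Blueprint activates the light, and its OnRightChoiceChosen event is empty.
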(event EventBeginPlay
  (|CallParentFunction)
  (Components|Activation|Deactivate (Variables|Default|GetPointLight)))

(event Collision|EventActorBeginOverlap
  (params (OtherActor :type Actor%20Object%20Reference)))

(event EventTick
  (params (DeltaSeconds :type Float%20%28single-precision%29))
  (bind _pointlight (Variables|Default|GetPointLight))
  (|CallParentFunction 0.0)
  (if (Components|Activation|IsActive (Variables|Default|GetPointLight))
    (Rendering|SetVisibility _pointlight true false)
    (else
      (Rendering|SetVisibility _pointlight false false))))

(event EventOnRightChoiceChosen)

(fn ConstructionScript
  (|CallParentFunction))