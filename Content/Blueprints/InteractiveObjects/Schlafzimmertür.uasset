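; Bedroom door ("Schlafzimmertür") interactive object, built as a child Blueprint that relies on its parent for setup and interaction logic.
; When the left choice is chosen, it runs the parent handler, then shows the left dialogue if that dialogue text is not empty.
; BeginPlay and the construction script only call the parent, and the overlap and Tick events are disabled.
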(event EventBeginPlay
  (|CallParentFunction))

(event Collision|EventActorBeginOverlap
  (params (OtherActor :type Actor%20Object%20Reference)))

(event EventTick
  (params (DeltaSeconds :type Float%20%28single-precision%29))
  (|CallParentFunction 0.0))

(event EventOnLeftChoiceChosen
  (|CallParentFunction)
  (if (not (Utilities|Text|TextIsEmpty (Variables|Default|GettextLeftInteractionDialogue)))
    (CallFunction|ShowLeftDialogue)))

(fn ConstructionScript
  (|CallParentFunction))