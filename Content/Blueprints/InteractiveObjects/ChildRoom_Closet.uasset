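; Interactive closet for the child's room with two hinged doors that toggle open and shut.
; A box overlap tracks whether the ChildFirstPersonCharacter is inside and enables input on the closet only during that time.
; Pressing Interact inside toggles the left door via the left-choice event.
; The right-choice event toggles the other door but is not called within this Blueprint; both snap hinge rotations and print debug text.
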(event OnComponentBeginOverlap(Box)
  (params (OverlappedComponent :type Primitive%20Component%20Object%20Reference) (OtherActor :type Actor%20Object%20Reference) (OtherComp :type Primitive%20Component%20Object%20Reference) (OtherBodyIndex :type Integer) (bFromSweep :type Boolean) (SweepResult :type Hit%20Result%20Structure%20%28by%20ref%29))
  ;[1 1 1] Is Player inside closet
  (Utilities|Casting|CastToChildFirstPersonCharacter OtherActor)
  (bind _output_get (Variables|Default|SetIsPlayerInside true))
  (Input|EnableInput (Game|GetPlayerController 0))
  (Development|PrintString (Class|KismetStringLibrary|BuildStringBool "Closet: Player Inside => " "" _output_get)))

(event OnComponentEndOverlap(Box)
  (params (OverlappedComponent :type Primitive%20Component%20Object%20Reference) (OtherActor :type Actor%20Object%20Reference) (OtherComp :type Primitive%20Component%20Object%20Reference) (OtherBodyIndex :type Integer))
  ;[1 1 1] Is Player inside closet
  (Utilities|Casting|CastToChildFirstPersonCharacter OtherActor)
  (bind _output_get (Variables|Default|SetIsPlayerInside false))
  (Input|DisableInput (Game|GetPlayerController 0))
  (Development|PrintString (Class|KismetStringLibrary|BuildStringBool "Closet: Player Inside => " "" _output_get)))

(event EventBeginPlay
  (|CallParentFunction))

(event Collision|EventActorBeginOverlap
  (params (OtherActor :type Actor%20Object%20Reference)))

(event EventTick
  (params (DeltaSeconds :type Float%20%28single-precision%29))
  (|CallParentFunction 0.0))

(event EventOnLeftChoiceChosen
  (bind _doorhingeleft (Variables|Default|GetDoorHingeLeft))
  ;[1 1 1] Left side choice
  (Development|PrintString "LeftDoor!")
  (if (Variables|Default|GetIsLeftDoorOpen)
    (Transformation|SetRelativeRotation _doorhingeleft "0.000000,0.000000,-90.000000" false false)
    (Variables|Default|SetIsLeftDoorOpen false)
    (else
      (Transformation|SetRelativeRotation _doorhingeleft "90.000000,0.000000,-90.000000" false false)
      (Variables|Default|SetIsLeftDoorOpen true))))

(event EventOnRightChoiceChosen
  (bind _doorhingeright (Variables|Default|GetDoorHingeRight))
  ;[1 1 1] Right side choice
  (Development|PrintString "RightDoor!")
  (if (Variables|Default|GetIsRightDoorOpen)
    (Transformation|SetRelativeRotation _doorhingeright "0, 0,-90.000000" false false)
    (Variables|Default|SetIsRightDoorOpen false)
    (else
      (Transformation|SetRelativeRotation _doorhingeright "-90.000000, 0,-90.000000" false false)
      (Variables|Default|SetIsRightDoorOpen true))))

(event Input|ActionEvents|InputActionInteract
  (params (Key :type Key%20Structure :default "AnyKey"))
  ;[1 1 1] Actual Interaction logic inside closet
  (:Pressed
    (if (Variables|Default|GetIsPlayerInside)
      (CallFunction|OnLeftChoiceChosen))))

(fn ConstructionScript
  (|CallParentFunction))