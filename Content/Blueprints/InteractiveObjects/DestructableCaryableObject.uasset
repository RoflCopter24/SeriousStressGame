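; Carryable interactive object that the player can smash via a left interaction (German prompt "Zerstören") once it becomes destructible.
; Tick catches Destructible turning true, swaps the static mesh for the destructible mesh and binds Destroy; the revert branch is unreachable.
; Destruct applies one-time radius damage at a zero-vector origin and sets Destroyed.
; Regret dialogue and pickup blocking apply only if Destroyed is already set during that transition.
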(event Custom|Destroy
  (CallFunction|Destruct))

(event EventBeginPlay
  (|CallParentFunction))

(event Collision|EventActorBeginOverlap
  (params (OtherActor :type Actor%20Object%20Reference)))

(event EventTick
  (params (DeltaSeconds :type Float%20%28single-precision%29))
  (bind _destructible (Variables|Default|GetDestructible))
  (|CallParentFunction DeltaSeconds)
  (if (and _destructible (not (Variables|Default|GetPreviouslyDestructable)))
    (if _destructible
      (Utilities|SetDestructibleComponentState true
        (:%20
          (Utilities|SetStaticMeshComponentState false
            (:%20
              (Variables|Default|SetbLeftInteraction true)
              (Variables|Default|SettextLeftInteraction "Zerstören")
              (EventDispatchers|BindEventtoOnLeftInteractionChosen (delegate Custom|Destroy))))))
      (else
        (Utilities|SetStaticMeshComponentState true
          (:%20
            (Utilities|SetDestructibleComponentState false
              (:%20
                (Variables|Default|SetbLeftInteraction false)
                (EventDispatchers|UnbindEventfromOnLeftInteractionChosen (delegate Custom|Destroy))))))))
    (if (Variables|Default|GetDestroyed)
      (Variables|Default|SettextRightInteractionDialogue "Ich hätte es nicht kaputt machen sollen. Aber ich war so wütend!")
      (Variables|Default|SetbLeftInteraction false)
      (Variables|Default|SetPickupBlocked true)))
  (Variables|Default|SetPreviouslyDestructable (Variables|Default|GetDestructible)))

(fn ConstructionScript
  (|CallParentFunction))

(fn Destruct
  (if (Variables|Default|GetDestructible)
    (if (Variables|Default|GetDestroyed)
      _
      (else
        (Class|DestructibleComponent|ApplyRadiusDamage (Variables|Default|GetDestructibleMesh) (Variables|Default|GetDamageApplied) (Math|Vector|MakeVector 0.0 0.0 0.0) (Variables|Default|GetDamageRadius) (Variables|Default|GetDamageStrength) true)
        (Variables|Default|SetDestroyed true))))
  (return))