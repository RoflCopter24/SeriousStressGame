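; Interactive toy Blueprint, apparently meant to be destructible, left as an unfinished stub.
; On BeginPlay it calls its parent and caches player 0's ChildFirstPersonCharacter as FpsController.
; The right-choice event and Destroy function are empty, and the Destructible mesh swap is never executed.
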(event EventBeginPlay
  (|CallParentFunction)
  (bind _aschild_first_person_character (Utilities|Casting|CastToChildFirstPersonCharacter (Game|GetPlayerCharacter 0)))
  (Variables|Default|SetFpsController _aschild_first_person_character))

(event Collision|EventActorBeginOverlap
  (params (OtherActor :type Actor%20Object%20Reference)))

(event EventTick
  (params (DeltaSeconds :type Float%20%28single-precision%29))
  (|CallParentFunction 0.0)
  (if true
    _))

(event EventOnRightChoiceChosen)

(fn ConstructionScript
  (|CallParentFunction))

(fn Destroy)