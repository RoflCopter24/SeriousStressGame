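; Interactive painting-table chair (Maltischstuhl) with two player choices: sit down or kick it.
; Left choice plays the sit sequence with player input disabled and the view switched to a named cine camera.
; Chained timers hold the pose, play the sequence in reverse, then restore input and the child character's view.
; Right choice snaps the mesh rotation based on Standing, with OnGround locking it and clearing the prompt once tipped.
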(event Custom|CustomEvent_0
  (Utilities|Time|SetTimerbyEvent (delegate Custom|CustomEvent_1) 15.0))

(event Custom|CustomEvent_1
  (bind _currentsequence (Variables|Default|GetCurrentSequence))
  (Components|Timeline|SetPlayRate _currentsequence -1.0)
  (Audio|Components|Audio|Play _currentsequence)
  (Utilities|Time|SetTimerbyEvent (delegate Custom|CustomEvent_2) (Class|LevelSequencePlayer|GetLength (Variables|Default|GetCurrentSequence))))

(event Custom|CustomEvent_2
  (bind _returnvalue (Game|GetPlayerController 0))
  (bind _asserious_stress_game_mode (Utilities|Casting|CastToSeriousStressGameMode (Game|GetGameMode)))
  (Default|EnablePlayerInput _asserious_stress_game_mode)
  (Variables|Default|SetSitting false)
  (bind _aschild_first_person_character (Utilities|Casting|CastToChildFirstPersonCharacter (Pawn|GetControlledPawn _returnvalue)))
  (Game|Player|SetViewTargetwithBlend _returnvalue _aschild_first_person_character 0.0 "VTBlend_Linear" 0.0 false) ; Switch view to camera actor
)

(event EventBeginPlay
  (|CallParentFunction))

(event Collision|EventActorBeginOverlap
  (params (OtherActor :type Actor%20Object%20Reference)))

(event EventOnRightChoiceChosen
  (bind _objectmesh (Variables|Default|GetObjectMesh))
  ;[1 1 1] right choice
  (if (Variables|Default|Getstanding)
    (if (not (Variables|Default|GetOnGround))
      (Transformation|SetRelativeRotation _objectmesh "0, 0,90.000000" false false)
      (Variables|Default|Setstanding false))
    (else
      (Transformation|SetRelativeRotation _objectmesh "85.000000,0.000000,90.000000" false false)
      (Variables|Default|Setstanding true)
      (Variables|Default|SetOnGround true)
      (Variables|Default|SettextRightInteraction ""))))

(event EventTick
  (params (DeltaSeconds :type Float%20%28single-precision%29))
  (|CallParentFunction 0.0))

(event EventOnLeftChoiceChosen
  (if (not (Variables|Default|GetSitting))
    (bind _returnvalue (Sequencer|Player|CreateLevelSequencePlayer "/Game/Animations/Seq_Maltisch_setzen.Seq_Maltisch_setzen"))
    (bind _output_get (Variables|Default|SetCurrentSequence _returnvalue))
    (Components|Timeline|SetPlayRate _output_get 1.0)
    (Audio|Components|Audio|Play _output_get)
    (bind _asserious_stress_game_mode (Utilities|Casting|CastToSeriousStressGameMode (Game|GetGameMode)))
    (Default|DisablePlayerInput _asserious_stress_game_mode)
    (Variables|Default|SetSitting true)
    (Utilities|Time|SetTimerbyEvent (delegate Custom|CustomEvent_0) (Class|LevelSequencePlayer|GetLength (Variables|Default|GetCurrentSequence)))
    (bind _asserious_stress_game_mode_2 (Utilities|Casting|CastToSeriousStressGameMode (Game|GetGameMode)))
    (bind _actor (Default|GetActorbyClassandName _asserious_stress_game_mode_2 "/Script/CinematicCamera.CineCameraActor" "CineCameraActor1_Setzen")) ; Get CineCameraActor
    (Game|Player|SetViewTargetwithBlend (Game|GetPlayerController 0) _actor 0.0 "VTBlend_Linear" 0.0 false) ; Switch view to camera actor
  ))

(fn ConstructionScript
  (|CallParentFunction))

(fn PlayCameraAnim)