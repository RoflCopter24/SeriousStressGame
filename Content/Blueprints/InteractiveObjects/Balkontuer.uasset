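; Interactive balcony door that the player opens and closes through an on-object interaction widget.
; It extends a parent interactable, showing or hiding the InteractionUI widget and filling in its enabled left and right options and their labels.
; BeginPlay binds to the widget's left-option click.
; The left choice shows its dialogue and toggles IsOpen, snapping the door between closed and open rotations without animation.
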(event EventBeginPlay
  (|CallParentFunction)
  (bind _asinteraction_ui (Utilities|Casting|CastToInteractionUI (UserInterface|GetUserWidgetObject (Variables|Default|GetWidget))))
  (EventDispatchers|BindEventtoOnOptionLeftClicked _asinteraction_ui (EventDispatchers|CreateEvent :!event OnLeftChoiceChosen)))

(event Collision|EventActorBeginOverlap
  (params (OtherActor :type Actor%20Object%20Reference)))

(event EventTick
  (params (DeltaSeconds :type Float%20%28single-precision%29))
  (|CallParentFunction 0.0))

(event EventOnLeftChoiceChosen
  (bind _tuer (Variables|Default|Gettuer))
  (CallFunction|ShowLeftDialogue)
  (if (Variables|Default|GetIsOpen)
    (Transformation|SetRelativeRotation _tuer "0, 0, 0" false false)
    (Variables|Default|SetIsOpen false)
    (else
      (Transformation|SetRelativeRotation _tuer "70.000000, 0, 0" false false)
      (Variables|Default|SetIsOpen true))))

(event EventShowInteractionUI
  (bind _widget (Variables|Default|GetWidget))
  (bind _returnvalue (UserInterface|GetUserWidgetObject _widget))
  ;[1 1 1] Show 2nd UI
  (|CallParentFunction)
  (Rendering|SetVisibility _widget true false)
  (Widget|SetVisibility _returnvalue "Visible")
  (bind _asinteraction_ui (Utilities|Casting|CastToInteractionUI _returnvalue))
  (if (Variables|Default|GetbLeftInteraction)
    (Default|EnableOptionLeft _asinteraction_ui))
  (if (Variables|Default|GetbRightInteraction)
    (Default|EnableOptionRight _asinteraction_ui))
  (Default|SetTextLeftOption _asinteraction_ui (Variables|Default|GettextLeftInteraction))
  (Default|SetTextRightOption _asinteraction_ui (Variables|Default|GettextRightInteraction)))

(event EventHideInteractionUI
  (bind _widget (Variables|Default|GetWidget))
  ;[1 1 1] Hide 2nd UI
  (|CallParentFunction)
  (Rendering|SetVisibility _widget false false)
  (Widget|SetVisibility (UserInterface|GetUserWidgetObject _widget) "Hidden"))

(fn ConstructionScript
  (|CallParentFunction))