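; Apartment door interactive object that offers a choice through its interaction widget and shows dialogue for the left option.
; On BeginPlay it runs the parent logic, casts the widget to InteractionUI and binds a handler to its left-option click.
; The OnLeftChoiceChosen event calls ShowLeftDialogue, while Tick and overlap events are disabled and construction only calls the parent.
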(event EventBeginPlay
  (|CallParentFunction)
  (bind _asinteraction_ui (Utilities|Casting|CastToInteractionUI (UserInterface|GetUserWidgetObject (Variables|Default|GetInteractionWidget))))
  (EventDispatchers|BindEventtoOnOptionLeftClicked _asinteraction_ui (EventDispatchers|CreateEvent :!event OnLeftChoiceChosen)))

(event Collision|EventActorBeginOverlap
  (params (OtherActor :type Actor%20Object%20Reference)))

(event EventTick
  (params (DeltaSeconds :type Float%20%28single-precision%29))
  (|CallParentFunction 0.0))

(event EventOnLeftChoiceChosen
  (CallFunction|ShowLeftDialogue))

(fn ConstructionScript
  (|CallParentFunction))