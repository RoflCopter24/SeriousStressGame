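; ClimbableChair is an interactive chair Blueprint that extends a parent pickup object.
; On BeginPlay it runs the parent logic, then hides its root scene component and all children.
; It overrides Pickup to call the parent implementation only while LockedToPosition is false, so a locked chair cannot be picked up.
; No climbing logic appears in this Blueprint, and its construction script only calls the parent.
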(event EventBeginPlay
  (|CallParentFunction)
  (Rendering|SetVisibility (Variables|Default|GetDefaultSceneRoot) false true))

(event Collision|EventActorBeginOverlap
  (params (OtherActor :type Actor%20Object%20Reference)))

(event EventTick
  (params (DeltaSeconds :type Float%20%28single-precision%29))
  (|CallParentFunction 0.0))

(event EventPickup
  (if (not (Variables|Default|GetLockedToPosition)) ; Allow pickup of object only when not locked
    (|CallParentFunction)))

(fn ConstructionScript
  (|CallParentFunction))