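; Interactive child's drawing (Kinderzeichnung) that blocks pickup on BeginPlay and offers a left/right choice on top of its parent class.
; The left choice shows the left dialogue, while the right choice destructs the object if it is Destructable.
; PlaySound assigns the sound cue to the audio component and plays it with the Open parameter off.
; Tick checks Destructable into a DoOnce that drives nothing further.
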(event EventBeginPlay
  (|CallParentFunction)
  (Variables|Default|SetPickupBlocked true))

(event Collision|EventActorBeginOverlap
  (params (OtherActor :type Actor%20Object%20Reference)))

(event EventTick
  (params (DeltaSeconds :type Float%20%28single-precision%29))
  (|CallParentFunction 0.0)
  (if (Variables|Default|GetDestructable)
    (Utilities|FlowControl|DoOnce false)))

(event EventOnLeftChoiceChosen
  (CallFunction|ShowLeftDialogue))

(event EventOnRightChoiceChosen
  (if (Variables|Default|GetDestructable)
    (CallFunction|Destruct)))

(fn ConstructionScript
  (|CallParentFunction))

(fn PlaySound
  (bind _audio (Variables|Default|GetAudio))
  (Audio|Components|Audio|SetSound _audio (Variables|Default|GetSoundCue))
  (Effects|Components|ParticleSystem|SetBoolParameter _audio "Open" false)
  (Audio|Components|Audio|Play _audio 0.0))