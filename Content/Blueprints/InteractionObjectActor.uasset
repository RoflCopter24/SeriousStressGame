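; Interactable world actor that tells the first-person character when it is close enough to interact with it.
; TriggerArea overlaps set the character's in-range state and store this actor as its InteractionObject, clearing both when the character leaves.
; The construction script binds an event to OnInteractDispatcher, and the OnInteract function is a placeholder that only prints a greeting.
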(event OnComponentBeginOverlap(TriggerArea)
  (params (OverlappedComponent :type Primitive%20Component%20Object%20Reference) (OtherActor :type Actor%20Object%20Reference) (OtherComp :type Primitive%20Component%20Object%20Reference) (OtherBodyIndex :type Integer) (bFromSweep :type Boolean) (SweepResult :type Hit%20Result%20Structure%20%28by%20ref%29))
  (Development|PrintText "In trigger Volume")
  (if (== (Utilities|GetClass OtherActor) "/Game/3rdParty/FirstPersonBP/Blueprints/FirstPersonCharacter.FirstPersonCharacter_C")
    (Variables|Default|SetPlayerInBounds true)
    (bind _asfirst_person_character (Utilities|Casting|CastToFirstPersonCharacter OtherActor))
    (Variables|/Game/3rdParty/FirstPersonBP/Blueprints/FirstPersonCharacter.FirstPersonCharacter_C|SetInInteractionRange _asfirst_person_character true)
    (Variables|/Game/3rdParty/FirstPersonBP/Blueprints/FirstPersonCharacter.FirstPersonCharacter_C|SetInteractionObject _asfirst_person_character self)
    (Default|SetinInteractionRange _asfirst_person_character true)))

(event OnComponentEndOverlap(TriggerArea)
  (params (OverlappedComponent :type Primitive%20Component%20Object%20Reference) (OtherActor :type Actor%20Object%20Reference) (OtherComp :type Primitive%20Component%20Object%20Reference) (OtherBodyIndex :type Integer))
  (if (== (Utilities|GetClass OtherActor) "/Game/3rdParty/FirstPersonBP/Blueprints/FirstPersonCharacter.FirstPersonCharacter_C")
    (Variables|Default|SetPlayerInBounds false)
    (bind _asfirst_person_character (Utilities|Casting|CastToFirstPersonCharacter OtherActor))
    (Variables|/Game/3rdParty/FirstPersonBP/Blueprints/FirstPersonCharacter.FirstPersonCharacter_C|SetInInteractionRange _asfirst_person_character false)
    (Default|SetinInteractionRange _asfirst_person_character false)
    (Variables|/Game/3rdParty/FirstPersonBP/Blueprints/FirstPersonCharacter.FirstPersonCharacter_C|SetInteractionObject _asfirst_person_character 0)))

(event EventBeginPlay)

(event Collision|EventActorBeginOverlap
  (params (OtherActor :type Actor%20Object%20Reference)))

(event EventTick
  (params (DeltaSeconds :type Float%20%28single-precision%29)))

(fn ConstructionScript
  (EventDispatchers|BindEventtoOnInteractDispatcher (EventDispatchers|CreateEvent :!event OnInteract)))

(fn OnInteract
  (Development|PrintString "Hello"))