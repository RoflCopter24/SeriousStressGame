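; Day 2 "BadFood" cutscene step, apparently unfinished: on creation it only hides the quest goal.
; The teleport and sequence creation sit on a dead branch, and playback and timers are disconnected; both sequence references name GoodFood assets.
; DialougeTrigger holds the father's German scolding about playing in the kitchen, and CutsceneFinished signals completion, but no live path here triggers either.
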(event Custom|CutsceneFinished
  (Default|CallOnCompleted))

(event Custom|DialougeTrigger
  ;[1 1 1] Dialouge Father
  (bind _dialogueuiinstance (CallFunction|CreateDialogueInstance 1))
  (Default|AddData _dialogueuiinstance 0 "Was ist hier passiert? Hast du dich verletzt? Du kannst doch nicht einfach so mit solch gefährlichen Sachen spielen! " 6.0)
  (Default|AddData _dialogueuiinstance 0 "Ich hab doch gesagt dass du aus der Küche draußen bleiben sollst. Das ist kein Ort zum Spielen! Was hätten ich und deine Mutter denn getan wenn du dich verletzt hättest? " 12.0)
  (Default|AddData _dialogueuiinstance 0 "Geh erst mal auf dein Zimmer. Ich räum die Unordnung auf und dann reden wir darüber. " 6.0))

(event EventCreated
  (CallFunction|HideQuestGoal)
  (if true
    (if true
      _)
    (else
      (Utilities|TeleportPlayer "PlayerStartName"
        (:Output
          (bind _newsequence (Default|CreateLevelSequencePlayer (Variables|Default|GetGameMode) "/Game/Animations/Cutscenes/Seq_Day2_03_GoodFood.Seq_Day2_03_GoodFood")))))))