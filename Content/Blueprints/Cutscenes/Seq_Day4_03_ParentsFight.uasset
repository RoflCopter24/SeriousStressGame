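; Cutscene script for Day 4 in which the parents come home and argue over the sister being locked out on the balcony.
; On creation it hides the quest goal, looks up the sister, father and mother characters by name, then plays the level sequence.
; Timers start the parents' argument and a later sibling exchange as separate dialogue instances, mostly voiced through each character's audio component.
; A timer matching the sequence length signals completion.
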(event Custom|CutsceneFinished
  (Default|CallOnCompleted))

(event Custom|Parentsfight
  (bind _father (Variables|Default|GetFather))
  (bind _mother (Variables|Default|GetMother))
  (bind _audio (Variables|/Game/Blueprints/Characters/InteractableCharacter.InteractableCharacter_C|GetAudio _father))
  (bind _audio_2 (Variables|/Game/Blueprints/Characters/InteractableCharacter.InteractableCharacter_C|GetAudio _mother))
  ;[1 1 1] Parents fight
  (bind _dialogueuiinstance (CallFunction|CreateDialogueInstance 2))
  (Default|AddData _dialogueuiinstance 0 "Ach das hat sie wirklich gesagt? Hahaha." 6.0 0 _audio)
  (Default|AddData _dialogueuiinstance 0 "Ja kannst du das fassen? Ich habs auch nicht glauben können." 6.0 0 _audio_2)
  (Default|AddData _dialogueuiinstance 0 "Euer Vater und ich hatten so einen schönen 	Morgen!" 6.0 0 _audio_2)
  (Default|AddData _dialogueuiinstance 0 "Wir wollten euch ausschlafen lassen deswegen sind wir so früh losgegangen. Geht es euch gut? Warum liegen hier denn überall Scherben rum?" 22.0 0 _audio_2)
  (Default|AddData _dialogueuiinstance 0 "Sie ist auf den Balkon gegangen und da ist 	der Blumentopf vor die Tür gefallen und sie war draußen ausgesperrt!" 18.0)
  (Default|AddData _dialogueuiinstance 0 "WAS ist passiert? Hättest du denn nicht besser auf sie aufpassen können?" 12.0 0 _audio_2)
  (Default|AddData _dialogueuiinstance 0 "Ich habe dir doch gesagt es ist eine schlechte Idee sie einfach alleine zu lassen!  Weßt du was ihr hätte passieren können?" 16.0 0 _audio_2)
  (Default|AddData _dialogueuiinstance 0 "Gibst du jetzt allen Ernstes mir die Schuld daran? Du wolltest doch ein tolles Frühstück und wir haben nun mal kein Babysitter 	gefunden. " 16.0 0 _audio)
  (Default|AddData _dialogueuiinstance 0 "Wir hatten doch einen schönen Morgen musst du dass jetzt ernsthaft deswegen kaputt machen? Es ist doch nichts passiert." 14.0 0 _audio)
  (Default|AddData _dialogueuiinstance 0 "Aber es hätte etwas passieren können? Und ich mache den Morgen kaputt?" 8.0 0 _audio_2)
  (Default|AddData _dialogueuiinstance 0 "Unsere Tochter hätte vom Balkon fallen können weil du so eine blöde Idee hast und ICH macheunseren Morgen kaputt? Verpiss dich doch!!" 16.0 0 _audio_2)
  (Default|AddData _dialogueuiinstance 0 "War ja klar dass das so kommen musste..." 6.0 0 _audio)
  (Default|AddData _dialogueuiinstance 0 "Ihr beide geht mal bitte auf euer Zimmer. Der Balkon ist ab sofort für euch Tabu! Habt ihr	mich verstanden?" 12.0 0 _audio))

(event Custom|DialougeTrigger
  ;[1 1 1] Sister-Brother-Conversation (after saving)
  (bind _dialogueuiinstance (CallFunction|CreateDialogueInstance 1))
  (Default|AddData _dialogueuiinstance 0 "Mamaaa...." 4.0 0 (Variables|/Game/Blueprints/Characters/InteractableCharacter.InteractableCharacter_C|GetAudio (Variables|Default|GetSister)))
  (Default|AddData _dialogueuiinstance 0 "Ich weiß, ich will auch das sie sich wieder lieb haben..." 8.0))

(event EventCreated
  (CallFunction|HideQuestGoal)
  (Utilities|GetSisterReference
    (:output
      (Utilities|GetFatherReference
        (:output
          (Utilities|GetMotherReference
            (:output
              (bind _newsequence (Default|CreateLevelSequencePlayer (Variables|Default|GetGameMode) "/Game/Animations/Cutscenes/Seq_Day4_03_ParentsFight.Seq_Day4_03_ParentsFight"))
              (Audio|Components|Audio|Play _newsequence)
              (Utilities|Time|SetTimerbyEvent (delegate Custom|CutsceneFinished) (Class|LevelSequencePlayer|GetLength _newsequence))
              (Utilities|Time|SetTimerbyEvent (delegate Custom|DialougeTrigger) 12.0)
              (Utilities|Time|SetTimerbyEvent (delegate Custom|Parentsfight) 4.0))))))))