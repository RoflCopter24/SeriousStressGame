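; Day 2 "GoodFood" cutscene, meant to show the father's German dialogue scolding the child after a kitchen mishap.
; As wired, Created only hides the quest goal: constant branches bypass the player teleport and creation of the Seq_Day2_03_GoodFood player.
; Playback and the timers for dialogue and completion are disconnected, so this graph never triggers the two dialogue lines or the completion callback.
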(event Custom|CutsceneFinished
  (Default|CallOnCompleted))

(event Custom|DialougeTrigger
  ;[1 1 1] Dialouge Father
  (bind _dialogueuiinstance (CallFunction|CreateDialogueInstance 1))
  (Default|AddData _dialogueuiinstance 0 "Was ist hier passiert? Hast du dich verletzt? Wieso hörst du denn nicht auf mich wenn ich dir sage dass du noch mit dem Essen wartensollst? " 12.0)
  (Default|AddData _dialogueuiinstance 0 "Die Küche kann ein sehr gefährlicher Ort für Kinder sein! Komm geh erst mal auf dein Zimmer und ich räum diese Unordnung auf. Aber hör das nächste Mal auf mich! Ich will mir keine Sorgen machen müssen!" 12.0))

(event EventCreated
  (CallFunction|HideQuestGoal)
  (if true
    (if true
      _)
    (else
      (Utilities|TeleportPlayer "Seq_Day2_04_PlayerStart"
        (:Output
          (bind _newsequence (Default|CreateLevelSequencePlayer (Variables|Default|GetGameMode) "/Game/Animations/Cutscenes/Seq_Day2_03_GoodFood.Seq_Day2_03_GoodFood")))))))