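; Day 1 cutscene 04-2 "toys on floor": the mother scolds the child about scattered toys, then the child reflects on the parents' fighting.
; On creation it hides the quest goal, teleports the player outside PIE, then plays the level sequence through a cine camera with input disabled.
; Hand-tuned timers trigger dialogues, an empty crying-sister stub and completion, which restores control.
; In PIE, a GameMode flag can skip it.
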(event Custom|CutsceneFinished
  (bind _gamemode (Variables|Default|GetGameMode))
  ;[1 1 1] Create Sequence Player, play sequence and set timer to fire after the length of that sequence
  (Default|CallOnCompleted)
  (Default|EnablePlayerInput _gamemode)
  (bind _player_controller (Default|GetPlayerControllerPub _gamemode))
  (Game|Player|SetViewTargetwithBlend _player_controller 0 0.5 "VTBlend_Linear" 0.0 false) ; Switch to default cam
)

(event Custom|CustomEvent_0
  ;[1 1 1] Show Cutscene in Editor?
  (Default|CallOnCompleted)
  (Development|PrintString 0 "Cutscene skipped 'cause of PIE!" true true "(R=1.000000,G=0.711824,B=0.000000,A=1.000000)"))

(event Custom|DialogueTrigger
  (bind _mother (Variables|Default|Getmother))
  (bind _audio (Variables|/Game/Blueprints/Characters/InteractableCharacter.InteractableCharacter_C|GetAudio _mother))
  ;[1 1 1] Dialog Mutter
  (bind _dialogueuiinstance (CallFunction|CreateDialogueInstance 1))
  (Default|AddData _dialogueuiinstance 0 "Was ist denn hier für eine Unordnung? Ich habe doch gesagt du sollst deine Spielsachen wegräumen!" 12.0 "/Game/Audio/Sounds/Characters/Mother/SC_Placeholder_Fight_Mother_single.SC_Placeholder_Fight_Mother_single" _audio)
  (Default|AddData _dialogueuiinstance 0 "Aber ich habe mein Spielzeug doch weggeräumt. " 6.0 "/Game/Audio/Sounds/Characters/Boy/SC_Placeholder_Child_single.SC_Placeholder_Child_single")
  (Default|AddData _dialogueuiinstance 0 "Das nennst du aufgeräumt? Es liegt hier doch überall herum! Man kann hier ja nirgendwo auftreten ohne etwas kaputtzumachen!" 12.0 "/Game/Audio/Sounds/Characters/Mother/SC_Placeholder_Fight_Mother_single.SC_Placeholder_Fight_Mother_single" _audio)
  (Default|AddData _dialogueuiinstance 0 "Räum diesen Saustall sofort auf sonst nehm ich dir alles weg und du bekommst nie wieder Spielzeug!" 12.0 "/Game/Audio/Sounds/Characters/Mother/SC_Placeholder_Fight_Mother_single.SC_Placeholder_Fight_Mother_single" _audio)
  (Default|AddData _dialogueuiinstance 0 "Verstanden?" 6.0 "/Game/Audio/Sounds/Characters/Mother/SC_Placeholder_Fight_Mother_single.SC_Placeholder_Fight_Mother_single" _audio)
  (Default|AddData _dialogueuiinstance 0 "... Ja." 6.0 "/Game/Audio/Sounds/Characters/Boy/SC_Placeholder_Child_single.SC_Placeholder_Child_single")
  (Default|Start _dialogueuiinstance))

(event Custom|DialogueTrigger_ChildThoughts
  ;[1 1 1] Junge wenn Mutter weg
  (bind _dialogueuiinstance (CallFunction|CreateDialogueInstance 1))
  (Default|AddData _dialogueuiinstance 0 "Mama ist immer so böse wenn sie und Papa sich gestritten haben..." 7.0 "/Game/Audio/Sounds/Characters/Boy/SC_Placeholder_Child_single.SC_Placeholder_Child_single")
  (Default|Start _dialogueuiinstance))

(event Custom|TriggerSound_CryingSister)

(event EventCreated
  (bind _gamemode (Variables|Default|GetGameMode))
  (bind _gamemode_2 (Variables|Default|GetGameMode))
  (CallFunction|HideQuestGoal)
  (if (Class|VictoryBPFunctionLibrary|WorldTypeinPIEWorld)
    ;[1 1 1] Show Cutscene in Editor?
    (if (Variables|/Game/Blueprints/GameState/SeriousStressGameMode.SeriousStressGameMode_C|GetCutscenesDuringPIE _gamemode)
      ;[1 1 1] Create Sequence Player, play sequence and set timer to fire after the length of that sequence
      (Default|DisablePlayerInputandLookatActor _gamemode :!label _label)
      (bind _newsequence (Default|CreateLevelSequencePlayer _gamemode "/Game/Animations/Cutscenes/Seq_Day1_04-2_ToysOnGround.Seq_Day1_04-2_ToysOnGround" (Utilities|Struct|MakeLevelSequencePlaybackSettings 0 1.0)))
      (Audio|Components|Audio|Play _newsequence)
      (Utilities|Time|SetTimerbyEvent (delegate Custom|CutsceneFinished) (Class|LevelSequencePlayer|GetLength _newsequence))
      (bind _player_controller (Default|GetPlayerControllerPub _gamemode_2))
      (bind _actor (Default|GetActorbyClassandName _gamemode_2 "/Script/CinematicCamera.CineCameraActor" "Seq_Day1_04_CameraActor")) ; Get CineCameraActor
      (Game|Player|SetViewTargetwithBlend _player_controller _actor 0.0 "VTBlend_Linear" 0.0 false) ; Switch view to camera actor
      (Utilities|Time|SetTimerbyEvent (delegate Custom|DialogueTrigger) 6.0) ; Zeiten an Level Sequence anpassen!!!
      (Utilities|Time|SetTimerbyEvent (delegate Custom|TriggerSound_CryingSister) 35.0)
      (Utilities|Time|SetTimerbyEvent (delegate Custom|DialogueTrigger_ChildThoughts) 54.0)
      (else
        (Utilities|Time|SetTimerbyEvent (delegate Custom|CustomEvent_0) 2.0)))
    (else
      (Utilities|TeleportPlayer "Seq_Day1_04_PlayerStart"
        (:Output
          (goto _label))))))