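; Cutscene script for Day 3 sequence 07-2, in which the boy argues with his mother about finding his sister's teddy and is sent to bed.
; On creation it shows the Briefe3 object and mother, plays the level sequence, attaches a separate hair actor to her socket and hides the crosshair.
; Timers start the voiced German dialogue, then on sequence end hide both actors, signal completion and restore the crosshair.
; Disabling detaches the hair for the next mother.
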(event Custom|OnSeqFinished
  ;[1 1 1] Objects visibility off
  (bind _motherreference (Utilities|GetMotherReference)
    (:Success
      (Rendering|SetVisibility (Variables|/Script/Engine.Character|GetMesh _motherreference) false false)
      (bind _interactableobjectbrief (Utilities|GetInteractableObjectReference)
        (:success
          (Rendering|SetVisibility (Variables|/Game/Blueprints/InteractiveObjects/InteractableObject.InteractableObject_C|GetObjectMesh _interactableobjectbrief) false false)
          (Default|CallOnCompleted)
          (Variables|/Game/Blueprints/GameState/SeriousStressGameMode.SeriousStressGameMode_C|SetDrawCrosshair (Variables|Default|GetGameMode) true))))))

(event Custom|Dialog
  (bind _mother (Variables|Default|GetMother))
  (bind _audio (Variables|/Game/Blueprints/Characters/InteractableCharacter.InteractableCharacter_C|GetAudio _mother))
  ;[1 1 1] Dialog
  (bind _childfpchar (CallFunction|GetPlayerCharRef))
  (bind _dialogueuiinstance (CallFunction|CreateDialogueInstance 1))
  (Default|AddData _dialogueuiinstance "/Game/Materials/DialougeImages/T_UI_DlgThumb_Boy_Brush.T_UI_DlgThumb_Boy_Brush" "..." 3.0)
  (Default|AddData _dialogueuiinstance "/Game/Materials/DialougeImages/T_UI_DlgThumb_Boy_Brush.T_UI_DlgThumb_Boy_Brush" "Mama, bist du da drinnen?" 6.0 "/Game/Audio/Sounds/Characters/Boy/SC_Placeholder_Child_single.SC_Placeholder_Child_single" (Variables|/Game/Blueprints/Characters/ChildFirstPersonCharacter.ChildFirstPersonCharacter_C|GetAudio _childfpchar))
  (Default|AddData _dialogueuiinstance "/Game/Materials/DialougeImages/T_UI_DlgThumb_Mother_Brush.T_UI_DlgThumb_Mother_Brush" "Warum bist du noch wach, du musst schon längst im Bett sein!" 8.0 "/Game/Audio/Sounds/Characters/Mother/SC_Placeholder_Fight_Mother_single.SC_Placeholder_Fight_Mother_single" _audio)
  (Default|AddData _dialogueuiinstance "/Game/Materials/DialougeImages/T_UI_DlgThumb_Boy_Brush.T_UI_DlgThumb_Boy_Brush" "Meine Schwester kann nicht schlafen, du musst ihren Teddy suchen!" 8.0 "/Game/Audio/Sounds/Characters/Boy/SC_Placeholder_Child_single.SC_Placeholder_Child_single" (Variables|/Game/Blueprints/Characters/ChildFirstPersonCharacter.ChildFirstPersonCharacter_C|GetAudio _childfpchar))
  (Default|AddData _dialogueuiinstance "/Game/Materials/DialougeImages/T_UI_DlgThumb_Mother_Brush.T_UI_DlgThumb_Mother_Brush" "Es ist schon spät, ich suche ihren Teddy jetzt nicht! Sie kann doch wohl eine Nacht ohne auskommen!" 12.0 "/Game/Audio/Sounds/Characters/Mother/SC_Placeholder_Fight_Mother_single.SC_Placeholder_Fight_Mother_single" _audio)
  (Default|AddData _dialogueuiinstance "/Game/Materials/DialougeImages/T_UI_DlgThumb_Boy_Brush.T_UI_DlgThumb_Boy_Brush" "Aber dann weint sie die ganze Nacht und dann kann ich nicht schlafen! Ich bin so müde!" 12.0 "/Game/Audio/Sounds/Characters/Boy/SC_Placeholder_Child_single.SC_Placeholder_Child_single" (Variables|/Game/Blueprints/Characters/ChildFirstPersonCharacter.ChildFirstPersonCharacter_C|GetAudio _childfpchar))
  (Default|AddData _dialogueuiinstance "/Game/Materials/DialougeImages/T_UI_DlgThumb_Mother_Brush.T_UI_DlgThumb_Mother_Brush" "Geh jetzt sofort ins Bett! Wir schauen morgen danach. Sie muss eine Nacht ohne auskommen!" 12.0 "/Game/Audio/Sounds/Characters/Mother/SC_Placeholder_Fight_Mother_single.SC_Placeholder_Fight_Mother_single" _audio)
  (Default|AddData _dialogueuiinstance "/Game/Materials/DialougeImages/T_UI_DlgThumb_Mother_Brush.T_UI_DlgThumb_Mother_Brush" "Sofort ins Bett! Ich will dich jetzt nicht mehr sehen!!" 8.0 "/Game/Audio/Sounds/Characters/Mother/SC_Placeholder_Fight_Mother_single.SC_Placeholder_Fight_Mother_single" _audio)
  (Default|Start _dialogueuiinstance))

(event EventCreated
  (bind _gamemode (Variables|Default|GetGameMode))
  (bind _interactableobjectbrief (Utilities|GetInteractableObjectReference)
    (:success
      (Rendering|SetVisibility (Variables|/Game/Blueprints/InteractiveObjects/InteractableObject.InteractableObject_C|GetObjectMesh _interactableobjectbrief) true false)
      (bind _motherreference (Utilities|GetMotherReference)
        (:Success
          (Rendering|SetVisibility (Variables|/Script/Engine.Character|GetMesh _motherreference) true false)
          (bind _newsequence (Default|CreateLevelSequencePlayer _gamemode "/Game/Animations/Cutscenes/Seq_Day3_07_2_Mother.Seq_Day3_07_2_Mother"))
          (Audio|Components|Audio|Play _newsequence)
          ;[1 1 1] MotherHair
          (bind _actor (Default|GetActorbyName (Variables|Default|GetGameMode) "MutterHaareOnly"))
          (bind _actor_2 (Default|GetActorbyName (Variables|Default|GetGameMode) "Day03-01_MotherChar"))
          (bind _asinteractable_character (Utilities|Casting|CastToInteractableCharacter _actor_2)
            (:then
              (Transformation|AttachComponentToComponent _actor (Variables|/Script/Engine.Character|GetMesh _asinteractable_character) "Hair" "SnapToTarget" "SnapToTarget" "SnapToTarget" true))
            (:CastFailed
              _))
          (Utilities|Time|SetTimerbyEvent (delegate Custom|OnSeqFinished) (Class|LevelSequencePlayer|GetLength _newsequence))
          (Variables|/Game/Blueprints/GameState/SeriousStressGameMode.SeriousStressGameMode_C|SetDrawCrosshair _gamemode false)
          (Utilities|Time|SetTimerbyEvent (delegate Custom|Dialog) 0.1))))))

(event EventDisabled
  ;[1 1 1] detach MotherHair for next Mother
  (bind _actor (Default|GetActorbyName (Variables|Default|GetGameMode) "MutterHaareOnly"))
  (Transformation|DetachFromActor _actor "KeepRelative" "KeepRelative" "KeepRelative"))