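; Cutscene object for the Day 4 monologue sequence, which plays a level sequence with a timed line of dialogue from the boy.
; On creation it has the GameMode create and play the sequence player, then sets a timer of the sequence's length to signal completion.
; A second fixed-delay timer starts a one-line dialogue instance with thumbnail and placeholder voice track, targeting the player character's audio component.
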(event Custom|CutsceneFinished
  (Default|CallOnCompleted))

(event Custom|DialougeTrigger
  ;[1 1 1] Monolog
  (bind _childfpchar (CallFunction|GetPlayerCharRef))
  (bind _dialogueuiinstance (CallFunction|CreateDialogueInstance 1))
  (Default|AddData _dialogueuiinstance "/Game/Materials/DialougeImages/T_UI_DlgThumb_Boy_Brush.T_UI_DlgThumb_Boy_Brush" "Warte hier. Ich schau mal nach was mit Mama los ist." 6.0 "/Game/Audio/Sounds/Characters/Boy/SC_Placeholder_Child_single.SC_Placeholder_Child_single" (Variables|/Game/Blueprints/Characters/ChildFirstPersonCharacter.ChildFirstPersonCharacter_C|GetAudio _childfpchar))
  (Default|Start _dialogueuiinstance))

(event EventCreated
  (bind _newsequence (Default|CreateLevelSequencePlayer (Variables|Default|GetGameMode) "/Game/Animations/Cutscenes/Seq_Day4_04-monolog.Seq_Day4_04-monolog"))
  (Audio|Components|Audio|Play _newsequence)
  (Utilities|Time|SetTimerbyEvent (delegate Custom|CutsceneFinished) (Class|LevelSequencePlayer|GetLength _newsequence))
  (Utilities|Time|SetTimerbyEvent (delegate Custom|DialougeTrigger) 12.0))