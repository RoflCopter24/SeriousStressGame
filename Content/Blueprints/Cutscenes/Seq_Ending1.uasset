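; Cutscene Blueprint for the first ending, which plays the Seq_ending1 level sequence.
; On creation it hides the quest goal, reveals five "Blatt" static meshes looked up by name, and signals completion through a timer matching the sequence length.
; A boy's German monologue about a family tragedy is built as timed dialogue lines in an event bound to a zero-second timer, which Unreal does not fire.
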(event Custom|CutsceneFinished
  (Default|CallOnCompleted))

(event Custom|dialog%20junge
  (bind _dialogueuiinstance (CallFunction|CreateDialogueInstance 1))
  (Default|AddData _dialogueuiinstance 0 "Nachdem es in letzter Zeit so viel Ärger zuhause gab, hat meine Mama mich irgendwann als Papa arbeiten war mit dem Fahrrad mitgenommen." 18.0)
  (Default|AddData _dialogueuiinstance 0 "Ich musste zu einem netten Mann gehen und ihm Sachen von mir erzählen. Wie es mir geht oder warum ich manchmal Sachen kaputtmache." 18.0)
  (Default|AddData _dialogueuiinstance 0 "Mama hat meine Schwester alleine zuhause gelassen weil sie dachte wir brauchen nicht lange. Aber als wir weg waren ist sie wieder auf den Balkon gegangen." 18.0)
  (Default|AddData _dialogueuiinstance 0 "Wir kamen gerade nach Hause als wir sie sahen..." 8.0)
  (Default|AddData _dialogueuiinstance 0 "..." 8.0))

(event EventCreated
  (CallFunction|HideQuestGoal)
  (Utilities|GetBlattbyname "Blatt" true
    (:success
      _)
    (:notfound
      _))
  (Utilities|GetBlattbyname "Blatt2" true
    (:success
      _)
    (:notfound
      _))
  (Utilities|GetBlattbyname "Blatt3" true
    (:success
      _)
    (:notfound
      _))
  (Utilities|GetBlattbyname "Blatt4" true
    (:success
      _)
    (:notfound
      _))
  (Utilities|GetBlattbyname "Blatt5" true
    (:success
      _)
    (:notfound
      _))
  (bind _newsequence (Default|CreateLevelSequencePlayer (Variables|Default|GetGameMode) "/Game/Animations/Cutscenes/seq_ending1.seq_ending1"))
  (Audio|Components|Audio|Play _newsequence)
  (Utilities|Time|SetTimerbyEvent (delegate Custom|CutsceneFinished) (Class|LevelSequencePlayer|GetLength _newsequence))
  (Utilities|Time|SetTimerbyEvent (delegate Custom|dialog%20junge) 0.0))