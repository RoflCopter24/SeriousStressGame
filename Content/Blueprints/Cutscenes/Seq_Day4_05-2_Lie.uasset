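; Day 4 cutscene in which the child's claim that Mother wants to reconcile sets off a German-language argument between the parents.
; On creation it hides the quest goal, finds both parent characters by name and plays the Level Sequence through the GameMode.
; A timer matching the sequence length signals completion.
; DialougeTrigger, bound to a zero-time timer, queues timed lines, most targeting the speaking parent's audio component.
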(event Custom|CutsceneFinished
  (Default|CallOnCompleted))

(event Custom|DialougeTrigger
  (bind _father (Variables|Default|GetFather))
  (bind _audio (Variables|/Game/Blueprints/Characters/InteractableCharacter.InteractableCharacter_C|GetAudio _father))
  ;[1 1 1] Dialouge Father
  (bind _dialogueuiinstance (CallFunction|CreateDialogueInstance 1))
  (Default|AddData _dialogueuiinstance 0 "Mama hat gesagt dass sie sich wieder mit dir Vertragen will... Du sollst zu ihr kommen und mit ihr reden. Ihr müsst euch entschuldigen." 12.0)
  (Default|AddData _dialogueuiinstance 0 "Ich soll mich bei IHR entschuldigen?! Es war genauso ihre Schuld!" 8.0 0 _audio)
  (Default|AddData _dialogueuiinstance 0 "" 3.0)
  (Default|AddData _dialogueuiinstance 0 "Was soll der Scheiß?! Ich soll mich bei dir entschuldigen? Fass dir mal an die eigene Nase!" 8.0 0 _audio)
  (Default|AddData _dialogueuiinstance 0 "Was redest du für ein Quatsch? Ich will mit dir kein Wort mehr reden! Verzieh dich gefälligst." 8.0 0 (Variables|/Game/Blueprints/Characters/InteractableCharacter.InteractableCharacter_C|GetAudio (Variables|Default|GetMother)))
  (Default|AddData _dialogueuiinstance 0 "Ja genau anstatt deinen Sohn zu schicken komm gefälligst selbst zu mir wenn du was zu sagen hast!" 8.0 0 _audio))

(event EventCreated
  (CallFunction|HideQuestGoal)
  (Utilities|GetFatherReference
    (:output
      (Utilities|GetMotherReference
        (:output
          (bind _newsequence (Default|CreateLevelSequencePlayer (Variables|Default|GetGameMode) "/Game/Animations/Cutscenes/Seq_Day4_05-2_Lie.Seq_Day4_05-2_Lie"))
          (Audio|Components|Audio|Play _newsequence)
          (Utilities|Time|SetTimerbyEvent (delegate Custom|CutsceneFinished) (Class|LevelSequencePlayer|GetLength _newsequence))
          (Utilities|Time|SetTimerbyEvent (delegate Custom|DialougeTrigger) 0.0))))))