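; Intro cutscene that, on creation, freezes the child player's tick and plays the intro level sequence with music and an overlay widget.
; A timer matching the sequence length restores tick, clears music and widget, and signals completion.
; In PIE, a GameMode flag can skip playback, completing after a short delay.
; It also reveals sister, father and mother NPCs, makes the mother angry, and clears the kick chair's RightInteraction flag.
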(event Custom|CutsceneFinished
  (Actor|Tick|SetActorTickEnabled (stale EventCreated _aschild_first_person_character) true)
  ;[1 1 1] music off
  (Audio|Components|Audio|Stop (Variables|Default|GetSound))
  (Default|CallOnCompleted)
  (Widget|RemovefromParent (stale EventCreated _widget_instance)))

(event Custom|CustomEvent_0
  (Actor|Tick|SetActorTickEnabled (stale EventCreated _aschild_first_person_character) true)
  (Default|CallOnCompleted))

(event EventCreated
  (bind _gamemode (Variables|Default|GetGameMode))
  (bind _gamemode_2 (Variables|Default|GetGameMode))
  (bind _actor (Default|GetActorbyClassandName _gamemode "/Game/Blueprints/Characters/ChildFirstPersonCharacter.ChildFirstPersonCharacter_C" "ChildFirstPersonCharacter"))
  (bind _aschild_first_person_character (Utilities|Casting|CastToChildFirstPersonCharacter _actor))
  (Actor|Tick|SetActorTickEnabled _aschild_first_person_character)
  (if (Class|VictoryBPFunctionLibrary|WorldTypeinPIEWorld)
    (if (Variables|/Game/Blueprints/GameState/SeriousStressGameMode.SeriousStressGameMode_C|GetCutscenesDuringPIE _gamemode)
      ;[1 1 1] music on
      (bind _output_get (Variables|Default|SetSound (Class|LowEntryExtendedStandardLibrary|CreateObject "/Script/Engine.AudioComponent") :!label _label))
      (Audio|Components|Audio|SetSound _output_get "/Game/Audio/Sounds/Start_Credit_Level/start_2_Cue.start_2_Cue")
      (Audio|Components|Audio|Play _output_get 0.0)
      (bind _newsequence (Default|CreateLevelSequencePlayer (Variables|Default|GetGameMode) "/Game/Animations/Cutscenes/Seq_Intro_alternative.Seq_Intro_alternative"))
      (Audio|Components|Audio|Play _newsequence)
      (bind _widget_instance (Default|CreateWidget (Variables|Default|GetGameMode) "/Game/Blueprints/UI/Intro.Intro_C"))
      (UserInterface|Viewport|AddtoViewport _widget_instance 0)
      (Utilities|Time|SetTimerbyEvent (delegate Custom|CutsceneFinished) (Class|LevelSequencePlayer|GetLength _newsequence))
      (else
        (Utilities|Time|SetTimerbyEvent (delegate Custom|CustomEvent_0) 0.5)))
    (else
      (goto _label)))
  (bind _actor_2 (Default|GetActorbyClassandName _gamemode_2 "/Game/Blueprints/Characters/InteractableCharacter.InteractableCharacter_C" "Quest_01-01_SisterChar"))
  (bind _asinteractable_character (Utilities|Casting|CastToInteractableCharacter _actor_2))
  (Default|EnableCollision _asinteractable_character)
  (Rendering|SetActorHiddenInGame _asinteractable_character false)
  (bind _actor_3 (Default|GetActorbyClassandName _gamemode_2 "/Game/Blueprints/Characters/InteractableCharacter.InteractableCharacter_C" "FatherChar_Day01-01"))
  (bind _asinteractable_character_2 (Utilities|Casting|CastToInteractableCharacter _actor_3))
  (Default|EnableCollision _asinteractable_character_2)
  (Rendering|SetActorHiddenInGame _asinteractable_character_2 false)
  (bind _actor_4 (Default|GetActorbyClassandName _gamemode_2 "/Game/Blueprints/Characters/InteractableCharacter.InteractableCharacter_C" "MotherChar_Day01-01"))
  (bind _asinteractable_character_3 (Utilities|Casting|CastToInteractableCharacter _actor_4))
  (Default|EnableCollision _asinteractable_character_3)
  (Rendering|SetActorHiddenInGame _asinteractable_character_3 false)
  (bind _actor_5 (Default|GetActorbyClassandName _gamemode_2 "/Game/Blueprints/Characters/InteractableCharacter.InteractableCharacter_C" "MotherChar_Day01-01"))
  (bind _asinteractable_character_4 (Utilities|Casting|CastToInteractableCharacter _actor_5))
  (bind _asabp_char_mother (Utilities|Casting|CastToABP_Char_Mother (Components|SkeletalMesh|GetAnimInstance (Variables|/Script/Engine.Character|GetMesh _asinteractable_character_4))))
  (Variables|/Game/Animations/Characters/ABP_Char_Mother.ABP_Char_Mother_C|SetIsAngry _asabp_char_mother true)
  (bind _actor_6 (Default|GetActorbyClassandName (Variables|Default|GetGameMode) "/Game/Blueprints/InteractiveObjects/Maltischstuhl_kick.Maltischstuhl_kick_C" "Maltischstuhl_kick"))
  (bind _asmaltischstuhl_kick (Utilities|Casting|CastToMaltischstuhl_kick _actor_6)
    (:then
      (Variables|/Game/Blueprints/InteractiveObjects/InteractableObject.InteractableObject_C|SetbRightInteraction _asmaltischstuhl_kick false))
    (:CastFailed
      (Development|PrintString 0 "WARNING: Maltischstuhl_kick not found!" true true "(R=1.000000,G=0.885502,B=0.000000,A=1.000000)"))))