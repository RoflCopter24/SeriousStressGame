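; Cutscene sequence Blueprint for the Day 4 intro, playing a level sequence with a time overlay widget and a German monologue from the boy.
; On creation it calls an empty scene-prop hook, adds the overlay, plays the sequence, then starts timers for the dialogue and the sequence end.
; The delayed dialogue queues three lines on the player character's audio component.
; When the sequence length elapses, it removes the overlay and signals completion.
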(event Custom|Seq_Done
  (Widget|RemovefromParent (stale EventCreated _widget_instance))
  (Default|CallOnCompleted))

(event Custom|DialogBoy
  ;[1 1 1] Dialouge Boy
  (bind _childfpchar (CallFunction|GetPlayerCharRef))
  (bind _dialogueuiinstance (CallFunction|CreateDialogueInstance))
  (Default|AddData _dialogueuiinstance 0 "Oh Mann was ist da schon wieder passiert? Ich dachte Mama und Papa sind nicht zu hause. Sie wollten ja heute irgendwo hin" 12.0 0 (Variables|/Game/Blueprints/Characters/ChildFirstPersonCharacter.ChildFirstPersonCharacter_C|GetAudio _childfpchar))
  (Default|AddData _dialogueuiinstance 0 "Bestimmt streiten sie wieder nur... Es ist schon irgendwie gruselig alleine zuhause. " 8.0 0 (Variables|/Game/Blueprints/Characters/ChildFirstPersonCharacter.ChildFirstPersonCharacter_C|GetAudio _childfpchar))
  (Default|AddData _dialogueuiinstance 0 "Ich sollte mal nachsehen was das für ein Geräusch war. Ich glaube es kam aus dem	Wohnzimmer." 12.0 0 (Variables|/Game/Blueprints/Characters/ChildFirstPersonCharacter.ChildFirstPersonCharacter_C|GetAudio _childfpchar))
  (Default|Start _dialogueuiinstance))

(event EventCreated
  (bind _gamemode (Variables|Default|GetGameMode))
  (CallFunction|ScenePropChange)
  (bind _widget_instance (Default|CreateWidget _gamemode "/Game/Blueprints/UI/Seq_Day4_01Intro_Timeoverlay.Seq_Day4_01Intro_Timeoverlay_C"))
  (UserInterface|Viewport|AddtoViewport _widget_instance 0)
  (bind _newsequence (Default|CreateLevelSequencePlayer _gamemode "/Game/Animations/Cutscenes/Seq_Day4_00_Intro.Seq_Day4_00_Intro"))
  (Audio|Components|Audio|Play _newsequence)
  (Utilities|Time|SetTimerbyEvent (delegate Custom|Seq_Done) (Class|LevelSequencePlayer|GetLength _newsequence))
  (Utilities|Time|SetTimerbyEvent (delegate Custom|DialogBoy) 6.0))

(event EventDisabled
  (CallFunction|OnDisabled))

(fn ScenePropChange
  (return))

(fn OnDisabled)