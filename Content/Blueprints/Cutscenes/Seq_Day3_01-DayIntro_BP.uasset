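; Cutscene object that plays the Day 3 intro level sequence and reports completion or cancellation.
; On creation it sets the light profile, teleports the player to the Day 3 start, plays the sequence with a time overlay and disables input.
; A length-based timer removes the overlay, restores input and shows the quest goal.
; Tick handles cancellation; the PIE skip branch is left unconnected.
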(event Custom|SequenceFinished
  (Development|PrintString 0 (Utilities|String|ToString(Float) (Class|LevelSequencePlayer|GetLength (stale EventCreated _newsequence))))
  (Widget|RemovefromParent (Variables|Default|GetWidget))
  (Default|EnablePlayerInput (Variables|Default|GetGameMode))
  (Default|CallOnCompleted)
  (CallFunction|ShowQuestGoal))

(event Custom|CustomEvent_0
  (Default|CallOnCanceled))

(event EventCreated
  (bind _gamemode (Variables|Default|GetGameMode))
  (Default|SetLightProfile (Variables|Default|GetGameMode) "NewEnumerator4")
  (if (Variables|/Game/Blueprints/GameState/SeriousStressGameMode.SeriousStressGameMode_C|GetCutscenesDuringPIE (Variables|Default|GetGameMode))
    _
    (elif (Class|VictoryBPFunctionLibrary|WorldTypeinPIEWorld)
      _
      (else
        _)))
  (bind _childfpcharacter (Utilities|GetPlayerCharRef)
    (:%20
      (bind _playerstarttransform (Utilities|GetStartLoc "Day03-01_PlayerStart")
        (:%20
          (Transformation|Teleport _childfpcharacter (.location _playerstarttransform) (.rotation _playerstarttransform))
          (bind _newsequence (Default|CreateLevelSequencePlayer _gamemode "/Game/Animations/Cutscenes/Seq_Day3_01-DayIntro.Seq_Day3_01-DayIntro"))
          (bind _output_get (Variables|Default|SetSequence _newsequence))
          (Audio|Components|Audio|Play _output_get)
          (bind _widget_instance (Default|CreateWidget _gamemode "/Game/Blueprints/UI/Seq_Day3_01Intro_Timeoverlay.Seq_Day3_01Intro_Timeoverlay_C"))
          (bind _output_get_2 (Variables|Default|SetWidget _widget_instance))
          (UserInterface|Viewport|AddtoViewport _output_get_2 0)
          (Utilities|Time|SetTimerbyEvent (delegate Custom|SequenceFinished) (Class|LevelSequencePlayer|GetLength _newsequence))
          (Default|DisablePlayerInput (Variables|Default|GetGameMode)))))))

(event EventTick
  (if (Variables|Default|GetCancel)
    (Audio|Components|Audio|Stop (Variables|Default|GetSequence))
    (Widget|RemovefromParent (Variables|Default|GetWidget))
    (Default|CallOnCanceled)
    (Default|EnablePlayerInput (Variables|Default|GetGameMode))))