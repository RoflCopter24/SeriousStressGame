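; Day 1 "Toys in Chest" cutscene Blueprint, in which the mother scolds the boy about toys lying around.
; On Created it attaches the shared hair actor to the mother, shows her, disables input and plays the level sequence, teleporting the player first outside PIE.
; Hand-timed timers trigger dialogues, an empty crying-sister stub and completion, which hides her and restores input.
; PIE skips playback unless CutscenesDuringPIE is set; Disabled detaches the hair.
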(event Custom|CutsceneFinished
  (bind _motherref (Utilities|GetMotherbyReference)
    (:Output
      (Rendering|SetVisibility (Variables|/Script/Engine.Character|GetMesh _motherref) false false)
      (Default|EnablePlayerInput (Variables|Default|GetGameMode))
      (Default|CallOnCompleted))))

(event Custom|CustomEvent_0
  (Default|CallOnCompleted)
  (Development|PrintString 0 "Cutscene skipped 'cause of PIE!" true true "(R=1.000000,G=0.711824,B=0.000000,A=1.000000)"))

(event Custom|DialogueTrigger
  (bind _mother (Variables|Default|GetMother))
  (bind _audio (Variables|/Game/Blueprints/Characters/InteractableCharacter.InteractableCharacter_C|GetAudio _mother))
  ;[1 1 1] Dialog Mutter
  (bind _childfpchar (CallFunction|GetPlayerCharRef))
  (bind _dialogueuiinstance (CallFunction|CreateDialogueInstance 1))
  (Default|AddData _dialogueuiinstance "/Game/Materials/DialougeImages/T_UI_DlgThumb_Mother_Brush.T_UI_DlgThumb_Mother_Brush" "Was habe ich dir vorhin gesagt?" 6.0 "/Game/Audio/Sounds/Characters/Mother/SC_Placeholder_Fight_Mother_single.SC_Placeholder_Fight_Mother_single" _audio)
  (Default|AddData _dialogueuiinstance "/Game/Materials/DialougeImages/T_UI_DlgThumb_Boy_Brush.T_UI_DlgThumb_Boy_Brush" "Dass ich mein Spielzeug aufräumen soll?" 6.0 "/Game/Audio/Sounds/Characters/Boy/SC_Placeholder_Child_single.SC_Placeholder_Child_single" (Variables|/Game/Blueprints/Characters/ChildFirstPersonCharacter.ChildFirstPersonCharacter_C|GetAudio _childfpchar))
  (Default|AddData _dialogueuiinstance "/Game/Materials/DialougeImages/T_UI_DlgThumb_Mother_Brush.T_UI_DlgThumb_Mother_Brush" "Ganz genau! Und warum liegt dann immer noch welches herum?" 6.0 "/Game/Audio/Sounds/Characters/Mother/SC_Placeholder_Fight_Mother_single.SC_Placeholder_Fight_Mother_single" _audio)
  (Default|AddData _dialogueuiinstance "/Game/Materials/DialougeImages/T_UI_DlgThumb_Boy_Brush.T_UI_DlgThumb_Boy_Brush" "Ich habe aber alles weggeräumt" 6.0 "/Game/Audio/Sounds/Characters/Boy/SC_Placeholder_Child_single.SC_Placeholder_Child_single" (Variables|/Game/Blueprints/Characters/ChildFirstPersonCharacter.ChildFirstPersonCharacter_C|GetAudio _childfpchar))
  (Default|AddData _dialogueuiinstance "/Game/Materials/DialougeImages/T_UI_DlgThumb_Boy_Brush.T_UI_DlgThumb_Boy_Brush" "..." 3.0 0 (Variables|/Game/Blueprints/Characters/ChildFirstPersonCharacter.ChildFirstPersonCharacter_C|GetAudio _childfpchar))
  (Default|AddData _dialogueuiinstance "/Game/Materials/DialougeImages/T_UI_DlgThumb_Boy_Brush.T_UI_DlgThumb_Boy_Brush" "...schau!" 4.0 "/Game/Audio/Sounds/Characters/Boy/SC_Placeholder_Child_single.SC_Placeholder_Child_single" (Variables|/Game/Blueprints/Characters/ChildFirstPersonCharacter.ChildFirstPersonCharacter_C|GetAudio _childfpchar))
  (Default|AddData _dialogueuiinstance "/Game/Materials/DialougeImages/T_UI_DlgThumb_Mother_Brush.T_UI_DlgThumb_Mother_Brush" "Ich habe unter dem Sofa noch welches gefunden! Wenn ich nochmal deine Spielsachen hier herumliegen sehe,.." 12.0 "/Game/Audio/Sounds/Characters/Mother/SC_Placeholder_Fight_Mother_single.SC_Placeholder_Fight_Mother_single" _audio)
  (Default|AddData _dialogueuiinstance "/Game/Materials/DialougeImages/T_UI_DlgThumb_Mother_Brush.T_UI_DlgThumb_Mother_Brush" "... dann nehme ich sie dir alle weg und du bekommst nie wieder welche! Hast du mich verstanden?" 12.0 "/Game/Audio/Sounds/Characters/Mother/SC_Placeholder_Fight_Mother_single.SC_Placeholder_Fight_Mother_single" _audio)
  (Default|AddData _dialogueuiinstance "/Game/Materials/DialougeImages/T_UI_DlgThumb_Boy_Brush.T_UI_DlgThumb_Boy_Brush" "..." 4.0)
  (Default|AddData _dialogueuiinstance "/Game/Materials/DialougeImages/T_UI_DlgThumb_Boy_Brush.T_UI_DlgThumb_Boy_Brush" "Ja." 4.0 "/Game/Audio/Sounds/Characters/Boy/SC_Placeholder_Child_single.SC_Placeholder_Child_single" (Variables|/Game/Blueprints/Characters/ChildFirstPersonCharacter.ChildFirstPersonCharacter_C|GetAudio _childfpchar))
  (Default|AddData _dialogueuiinstance "/Game/Materials/DialougeImages/T_UI_DlgThumb_Mother_Brush.T_UI_DlgThumb_Mother_Brush" "Und jetzt räum sie weg bevor dein Vater kommt und hier noch mehr Stress veranstaltet!" 12.0 "/Game/Audio/Sounds/Characters/Mother/SC_Placeholder_Fight_Mother_single.SC_Placeholder_Fight_Mother_single" _audio)
  (Default|Start _dialogueuiinstance))

(event Custom|DialogueTrigger_ChildThoughts
  ;[1 1 1] Junge wenn Mutter weg
  (bind _childfpchar (CallFunction|GetPlayerCharRef))
  (bind _dialogueuiinstance (CallFunction|CreateDialogueInstance 1))
  (Default|AddData _dialogueuiinstance "/Game/Materials/DialougeImages/T_UI_DlgThumb_Boy_Brush.T_UI_DlgThumb_Boy_Brush" "Mama ist immer so böse wenn sie und Papa sich gestritten haben..." 6.0 "/Game/Audio/Sounds/Characters/Boy/SC_Placeholder_Child_single.SC_Placeholder_Child_single" (Variables|/Game/Blueprints/Characters/ChildFirstPersonCharacter.ChildFirstPersonCharacter_C|GetAudio _childfpchar))
  (Default|Start _dialogueuiinstance))

(event Custom|TriggerSound_CryingSister)

(event EventCreated
  (bind _gamemode (Variables|Default|GetGameMode))
  ;[1 1 1] MotherHair
  (bind _actor (Default|GetActorbyName (Variables|Default|GetGameMode) "MutterHaareOnly"))
  (bind _actor_2 (Default|GetActorbyName (Variables|Default|GetGameMode) "Day01_02_MotherCharacter"))
  (bind _asinteractable_character (Utilities|Casting|CastToInteractableCharacter _actor_2))
  (Transformation|AttachComponentToComponent _actor (Variables|/Script/Engine.Character|GetMesh _asinteractable_character) "Hair" "SnapToTarget" "SnapToTarget" "SnapToTarget" true)
  (bind _motherref (Utilities|GetMotherbyReference)
    (:Output
      (Rendering|SetVisibility (Variables|/Script/Engine.Character|GetMesh _motherref) true false)
      (if (Class|VictoryBPFunctionLibrary|WorldTypeinPIEWorld)
        (if (Variables|/Game/Blueprints/GameState/SeriousStressGameMode.SeriousStressGameMode_C|GetCutscenesDuringPIE _gamemode)
          (bind _newsequence (Default|CreateLevelSequencePlayer _gamemode "/Game/Animations/Cutscenes/Seq_Day1_04-1_ToysInChest.Seq_Day1_04-1_ToysInChest" :!label _label))
          (Audio|Components|Audio|Play _newsequence)
          (Default|DisablePlayerInput (Variables|Default|GetGameMode))
          (Utilities|Time|SetTimerbyEvent (delegate Custom|CutsceneFinished) (Class|LevelSequencePlayer|GetLength _newsequence))
          (Utilities|Time|SetTimerbyEvent (delegate Custom|DialogueTrigger) 6.0) ; Zeiten an Level Sequence anpassen!!!
          (Utilities|Time|SetTimerbyEvent (delegate Custom|TriggerSound_CryingSister) 5e+01)
          (Utilities|Time|SetTimerbyEvent (delegate Custom|DialogueTrigger_ChildThoughts) 75.0)
          (else
            (Utilities|Time|SetTimerbyEvent (delegate Custom|CustomEvent_0) 1.0)))
        (else
          (Utilities|TeleporttoPlayerStart "Seq_Day1_04_PlayerStart"
            (:Output
              (goto _label))))))))

(event EventDisabled
  ;[1 1 1] detach MotherHair for next Mother
  (bind _actor (Default|GetActorbyName (Variables|Default|GetGameMode) "MutterHaareOnly"))
  (Transformation|DetachFromActor _actor "KeepRelative" "KeepRelative" "KeepRelative"))