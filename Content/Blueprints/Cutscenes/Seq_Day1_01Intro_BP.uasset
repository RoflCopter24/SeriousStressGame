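; Day 1 intro cutscene Blueprint that plays the Seq_Day1_01Intro level sequence with a time overlay widget.
; On creation it builds a sequence player through the GameMode, then uses timers to start a short German dialogue line mid-sequence and signal completion after the sequence length.
; In PIE, unless the GameMode enables cutscenes, it skips playback and signals completion after a brief delay.
; An older lookup of a placed sequence actor remains unconnected.
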(event Custom|CutsceneFinished
  (Default|CallOnCompleted))

(event Custom|CustomEvent_0
  (Default|CallOnCompleted)
  (Development|PrintString 0 "Cutscene skipped 'cause of PIE!" true true "(R=1.000000,G=0.711824,B=0.000000,A=1.000000)"))

(event Custom|DialogueTrigger
  (bind _dialogueuiinstance (CallFunction|CreateDialogueInstance 1))
  (Default|AddData _dialogueuiinstance 0 "Hm? Was ist da los?" 5.0)
  (Default|Start _dialogueuiinstance))

(event EventCreated
  (bind _gamemode (Variables|Default|GetGameMode))
  (if (Class|VictoryBPFunctionLibrary|WorldTypeinPIEWorld)
    (if (Variables|/Game/Blueprints/GameState/SeriousStressGameMode.SeriousStressGameMode_C|GetCutscenesDuringPIE _gamemode)
      (bind _newsequence (Default|CreateLevelSequencePlayer _gamemode "/Game/Animations/Cutscenes/Seq_Day1_01Intro.Seq_Day1_01Intro" (Utilities|Struct|MakeLevelSequencePlaybackSettings 0 1.0) :!label _label))
      (Components|Timeline|SetPlaybackPosition _newsequence 0.0)
      (Audio|Components|Audio|Play (Variables|/Script/LevelSequence.LevelSequenceActor|GetSequencePlayer (stale _output_get)))
      (bind _widget_instance (Default|CreateWidget (Variables|Default|GetGameMode) "/Game/Blueprints/UI/Seq_Day1_01Intro_Timeoverlay.Seq_Day1_01Intro_Timeoverlay_C"))
      (UserInterface|Viewport|AddtoViewport _widget_instance 0)
      (Utilities|Time|SetTimerbyEvent (delegate Custom|CutsceneFinished) (Class|LevelSequencePlayer|GetLength _newsequence))
      (Utilities|Time|SetTimerbyEvent (delegate Custom|DialogueTrigger) 6.0)
      (else
        (Utilities|Time|SetTimerbyEvent (delegate Custom|CustomEvent_0) 2.0)))
    (else
      (goto _label))))