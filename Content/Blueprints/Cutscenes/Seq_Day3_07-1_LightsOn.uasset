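; Cutscene Blueprint for the Day 3 "07-1 LightsOn" sequence, in which the mother scolds the child for being out of bed.
; On creation it hides the quest goal, shows two toys and the mother looked up by name, then plays the level sequence.
; A short timer starts the subtitled German dialogue with placeholder voice tracks.
; A timer matching the sequence length hides those actors again and calls OnCompleted.
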(event Custom|OnSeqFinished
  ;[1 1 1] Object Visibility OFF
  (bind _motherref (Utilities|GetMotherReference)
    (:success
      (Rendering|SetVisibility (Variables|/Script/Engine.Character|GetMesh _motherref) false false)
      (bind _interactableobject (Utilities|GetInteractableObjectReference "car_toy_3")
        (:success
          (Rendering|SetVisibility (Variables|/Game/Blueprints/InteractiveObjects/InteractableObject.InteractableObject_C|GetObjectMesh _interactableobject) false false)
          (bind _interactableobject_2 (Utilities|GetInteractableObjectReference "Quest_Toy_DinoPlueschtier2")
            (:success
              (Rendering|SetVisibility (Variables|/Game/Blueprints/InteractiveObjects/InteractableObject.InteractableObject_C|GetObjectMesh _interactableobject_2) false false)
              (Default|CallOnCompleted))))))))

(event Custom|Dialouge
  (bind _mother (Variables|Default|GetMother))
  (bind _audio (Variables|/Game/Blueprints/Characters/InteractableCharacter.InteractableCharacter_C|GetAudio _mother))
  ;[1 1 1] Dialog
  (bind _dialogueuiinstance (CallFunction|CreateDialogueInstance 1))
  (Default|AddData _dialogueuiinstance 0 "Endlich hab ich dich gefunden du doofes Ding... Ich krieg noch ärger wegen dir..." 8.0 "/Game/Audio/Sounds/Characters/Boy/SC_Placeholder_Child_single.SC_Placeholder_Child_single")
  (Default|AddData _dialogueuiinstance 0 "Was zum Teufel machst du hier, du sollst längst im Bett sein!" 8.0 "/Game/Audio/Sounds/Characters/Mother/SC_Placeholder_Fight_Mother_single.SC_Placeholder_Fight_Mother_single" _audio)
  (Default|AddData _dialogueuiinstance 0 "Sie hat geweint und ich wollte ihren Teddy haben, ich hab ihn nur gesucht." 8.0 "/Game/Audio/Sounds/Characters/Boy/SC_Placeholder_Child_single.SC_Placeholder_Child_single")
  (Default|AddData _dialogueuiinstance 0 "Erzähl mir doch keinen Quatsch. Sie schläft doch sicher schon längst. Für euch ist schon längst Schlafenszeit! " 14.0 "/Game/Audio/Sounds/Characters/Mother/SC_Placeholder_Fight_Mother_single.SC_Placeholder_Fight_Mother_single" _audio)
  (Default|AddData _dialogueuiinstance 0 "Maschier sofort ins Bett!" 8.0 "/Game/Audio/Sounds/Characters/Mother/SC_Placeholder_Fight_Mother_single.SC_Placeholder_Fight_Mother_single" _audio)
  (Default|AddData _dialogueuiinstance 0 "Was soll das denn? Jetzt hast du bestimmt deine Schwester aufgeweckt! Geh sofort ins Bett!!" 14.0 "/Game/Audio/Sounds/Characters/Mother/SC_Placeholder_Fight_Mother_single.SC_Placeholder_Fight_Mother_single" _audio)
  (Default|Start _dialogueuiinstance))

(event EventCreated
  (CallFunction|HideQuestGoal)
  ;[1 1 1] Object Visibility ON
  (bind _interactableobject (Utilities|GetInteractableObjectReference "car_toy_3")
    (:success
      (Rendering|SetVisibility (Variables|/Game/Blueprints/InteractiveObjects/InteractableObject.InteractableObject_C|GetObjectMesh _interactableobject) true false)
      (bind _interactableobject_2 (Utilities|GetInteractableObjectReference "Quest_Toy_DinoPlueschtier2")
        (:success
          (Rendering|SetVisibility (Variables|/Game/Blueprints/InteractiveObjects/InteractableObject.InteractableObject_C|GetObjectMesh _interactableobject_2) true false)
          (bind _motherref (Utilities|GetMotherReference)
            (:success
              (Rendering|SetVisibility (Variables|/Script/Engine.Character|GetMesh _motherref) true false)
              (bind _newsequence (Default|CreateLevelSequencePlayer (Variables|Default|GetGameMode) "/Game/Animations/Cutscenes/Seq_Day3_07_1_LightsOn.Seq_Day3_07_1_LightsOn"))
              (Audio|Components|Audio|Play _newsequence)
              (Utilities|Time|SetTimerbyEvent (delegate Custom|OnSeqFinished) (Class|LevelSequencePlayer|GetLength _newsequence))
              (Utilities|Time|SetTimerbyEvent (delegate Custom|Dialouge) 0.01))))))))

(event EventTick)