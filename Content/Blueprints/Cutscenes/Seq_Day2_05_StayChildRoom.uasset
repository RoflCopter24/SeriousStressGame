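; Day 2 cutscene step for the stay-in-child-room scene, where the mother scolds her child for noisy play.
; On creation it hides the quest goal, teleports the player to a named PlayerStart, finds the mother character and plays level sequence Seq_Day2_04_StayCR.
; A zero-delay timer starts the hardcoded German dialogue, with placeholder voice on the mother's audio component.
; A timer matching the sequence length signals completion, independent of dialogue length.
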(event Custom|CutsceneFinished
  (Default|CallOnCompleted))

(event Custom|DialougeTrigger
  (bind _mother (Variables|Default|Getmother))
  (bind _audio (Variables|/Game/Blueprints/Characters/InteractableCharacter.InteractableCharacter_C|GetAudio _mother))
  ;[1 1 1] Dialouge Mother
  (bind _dialogueuiinstance (CallFunction|CreateDialogueInstance 1))
  (Default|AddData _dialogueuiinstance 0 "Brumm! Brumm!" 6.0)
  (Default|AddData _dialogueuiinstance 0 "Musst du immer so laut sein beim Spielen? Kannst du nicht mal leise sein, wie deine Schwester? Ich brauche auch mal meine Ruhe!" 16.0 "/Game/Audio/Sounds/Characters/Mother/SC_Placeholder_Fight_Mother_single.SC_Placeholder_Fight_Mother_single" _audio)
  (Default|AddData _dialogueuiinstance 0 "Mama, warum weinst du?" 6.0)
  (Default|AddData _dialogueuiinstance 0 "Es ist nichts! Geh und spiel mit deiner Schwester. Aber sei um Gottes willen leise!! " 8.0 "/Game/Audio/Sounds/Characters/Mother/SC_Placeholder_Fight_Mother_single.SC_Placeholder_Fight_Mother_single" _audio)
  (Default|Start _dialogueuiinstance))

(event EventCreated
  (CallFunction|HideQuestGoal)
  (Utilities|TeleportPlayer "Day01_02_PlayerStart"
    (:Output
      (Utilities|Getmotherreference
        (:Output
          (bind _newsequence (Default|CreateLevelSequencePlayer (Variables|Default|GetGameMode) "/Game/Animations/Cutscenes/Seq_Day2_04_StayCR.Seq_Day2_04_StayCR"))
          (Audio|Components|Audio|Play _newsequence)
          (Utilities|Time|SetTimerbyEvent (delegate Custom|CutsceneFinished) (Class|LevelSequencePlayer|GetLength _newsequence))
          (Utilities|Time|SetTimerbyEvent (delegate Custom|DialougeTrigger) 0.0))))))