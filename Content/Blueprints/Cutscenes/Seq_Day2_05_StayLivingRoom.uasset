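; Day 2 living-room cutscene in which the crying mother snaps at her child and sends them to their room.
; On creation it hides the quest goal, shows the named mother character and plays a level sequence, with timers triggering the German placeholder-voiced dialogue and flagging sequence end.
; Tick waits for both sequence and dialogue to finish, then hides the mother and calls completion.
; A TeleportPlayer helper is defined but unused.
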(event Custom|CutsceneFinished
  (Variables|Default|SetSeqComplete true))

(event Custom|DialougeTrigger
  (bind _mother (Variables|Default|Getmother))
  (bind _audio (Variables|/Game/Blueprints/Characters/InteractableCharacter.InteractableCharacter_C|GetAudio _mother))
  ;[1 1 1] Dialouge Mother
  (bind _dialogueuiinstance (CallFunction|CreateDialogueInstance 2))
  (Default|AddData _dialogueuiinstance 0 "Warum musst du  hier so rumtoben? Siehst du nicht das ich einen Moment für mich brauche?" 8.0 "/Game/Audio/Sounds/Characters/Mother/SC_Placeholder_Fight_Mother_single.SC_Placeholder_Fight_Mother_single" _audio)
  (Default|AddData _dialogueuiinstance 0 "Geh sofort auf dein Zimmer und Spiel da. Ich brauch auch mal eine Pause! Wieso bekomme ich nie eine Pause?." 8.0 "/Game/Audio/Sounds/Characters/Mother/SC_Placeholder_Fight_Mother_single.SC_Placeholder_Fight_Mother_single" _audio)
  (Default|AddData _dialogueuiinstance 0 "Mama, warum weinst du?" 6.0 "/Game/Audio/Sounds/Characters/Boy/SC_Placeholder_Child_single.SC_Placeholder_Child_single")
  (Default|AddData _dialogueuiinstance 0 "Es ist nichts! Geh jetzt sofort zu deiner Schwester aufs Zimmer und sei leise!" 8.0 "/Game/Audio/Sounds/Characters/Mother/SC_Placeholder_Fight_Mother_single.SC_Placeholder_Fight_Mother_single" _audio)
  (bind _output_get (Variables|Default|SetDlgInstance _dialogueuiinstance))
  (Default|Start _output_get))

(event EventTick
  ;[1 1 1] Check if Seq has finished
  (if (Variables|Default|GetSeqComplete)
    ;[1 1 1] If Seq is finished, make sure to wait until Dialogue has finished
    (bind _dlginstance (Variables|Default|GetDlgInstance)
      (:then
        (if (Variables|/Game/Blueprints/UI/DialogueUi.DialogueUi_C|GetbFinished _dlginstance)
          ;[1 1 1] MothercharacterVisibility
          (bind _mothercharacterreference (Utilities|Getmotherreference)
            (:output
              (Rendering|SetVisibility (Variables|/Script/Engine.Character|GetMesh _mothercharacterreference) false false)
              (Default|CallOnCompleted)))))
      (:else))))

(event EventCreated
  (CallFunction|HideQuestGoal)
  (bind _mothercharacterreference (Utilities|Getmotherreference)
    (:output
      (Rendering|SetVisibility (Variables|/Script/Engine.Character|GetMesh _mothercharacterreference) true false)
      (bind _newsequence (Default|CreateLevelSequencePlayer (Variables|Default|GetGameMode) "/Game/Animations/Cutscenes/Seq_Day2_04_StayLR.Seq_Day2_04_StayLR"))
      (Audio|Components|Audio|Play _newsequence)
      (Utilities|Time|SetTimerbyEvent (delegate Custom|CutsceneFinished) (Class|LevelSequencePlayer|GetLength _newsequence))
      (Utilities|Time|SetTimerbyEvent (delegate Custom|DialougeTrigger) 0.1))))