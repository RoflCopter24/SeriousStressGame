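; Day 4 "Truth" cutscene: the child tells Father that Mother wants him out, and the parents break into a fight.
; On creation it hides the quest goal, finds both parents by actor name, shows their meshes and plays the level sequence.
; A short timer starts the German dialogue chain with placeholder voice tracks, the parents' lines using their audio components.
; A timer matching the sequence length re-shows both meshes and signals completion.
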(event Custom|CutsceneFinished
  (bind _mothercharacterreference (Utilities|GetMotherReference)
    (:output
      (Rendering|SetVisibility (Variables|/Script/Engine.Character|GetMesh _mothercharacterreference) true false)
      (bind _fathercharacterreference (Utilities|GetFatherreference)
        (:output
          (Rendering|SetVisibility (Variables|/Script/Engine.Character|GetMesh _fathercharacterreference) true false)
          (Default|CallOnCompleted))))))

(event Custom|DialougeTrigger
  (bind _father (Variables|Default|GetFather))
  (bind _audio (Variables|/Game/Blueprints/Characters/InteractableCharacter.InteractableCharacter_C|GetAudio _father))
  ;[1 1 1] Dialouge Father
  (bind _dialogueuiinstance (CallFunction|CreateDialogueInstance 1))
  (Default|AddData _dialogueuiinstance 0 "Mama hat gesagt dass du hier nicht mehr sein darfst. Du sollst dir einen anderen Platz zum Schlafen suchen... Papa kannst du nicht hier...." 18.0 "/Game/Audio/Sounds/Characters/Boy/SC_Placeholder_Child_single.SC_Placeholder_Child_single")
  (Default|AddData _dialogueuiinstance 0 "Was hat sie gesagt?!" 6.0 "/Game/Audio/Sounds/Characters/Father/SC_Placeholder_Fight_Father_single.SC_Placeholder_Fight_Father_single" _audio)
  (Default|AddData _dialogueuiinstance 0 "" 3.0)
  (Default|AddData _dialogueuiinstance 0 "Du willst mich aus meiner eigenen Wohnung schmeißen? Wegen so einem dummen Unfall? Das kann doch jedem mal passieren! Ich verstehe nicht warum du dich wieder so aufregst!" 22.0 "/Game/Audio/Sounds/Characters/Father/SC_Placeholder_Fight_Father_single.SC_Placeholder_Fight_Father_single" _audio)
  (Default|AddData _dialogueuiinstance 0 "Du kannst machen was du willst? Wie wärs wenn du mal was im Haus tust anstatt nur vor der Glotze zu hängen? Du zerreißt den 						Familienzusammenhalt! Und jetzt bringst du auch noch unsere Kinder in Gefahr!" 22.0 "/Game/Audio/Sounds/Characters/Mother/SC_Placeholder_Fight_Mother_single.SC_Placeholder_Fight_Mother_single" (Variables|/Game/Blueprints/Characters/InteractableCharacter.InteractableCharacter_C|GetAudio (Variables|Default|GetMother)))
  (Default|AddData _dialogueuiinstance 0 "Ich zerreiße diese Familie? Du gibst doch auch keinen Scheiß mehr auf die Kinder. Du wolltest doch genauso mal ohne sie raus!" 12.0 "/Game/Audio/Sounds/Characters/Father/SC_Placeholder_Fight_Father_single.SC_Placeholder_Fight_Father_single" _audio)
  (Default|Start _dialogueuiinstance))

(event EventCreated
  (CallFunction|HideQuestGoal)
  (bind _mothercharacterreference (Utilities|GetMotherReference)
    (:output
      (Rendering|SetVisibility (Variables|/Script/Engine.Character|GetMesh _mothercharacterreference) true false)
      (bind _fathercharacterreference (Utilities|GetFatherreference)
        (:output
          (Rendering|SetVisibility (Variables|/Script/Engine.Character|GetMesh _fathercharacterreference) true false)
          (bind _newsequence (Default|CreateLevelSequencePlayer (Variables|Default|GetGameMode) "/Game/Animations/Cutscenes/Seq_Day4_05_1-Truth.Seq_Day4_05_1-Truth"))
          (Audio|Components|Audio|Play _newsequence)
          (Utilities|Time|SetTimerbyEvent (delegate Custom|CutsceneFinished) (Class|LevelSequencePlayer|GetLength _newsequence))
          (Utilities|Time|SetTimerbyEvent (delegate Custom|DialougeTrigger) 0.2))))))