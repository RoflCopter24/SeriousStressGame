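; Cutscene step for the second ending: plays its level sequence with an Ending2 widget on screen.
; On creation it hides the quest goal and reveals paper meshes Blatt6 to Blatt10, looked up by actor name.
; A timer matching the sequence length signals completion and removes the widget.
; A German dialogue in which a boy recounts leaving his sister alone is defined, but its trigger timer is disconnected.
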(event Custom|CutsceneFinished
  (Default|CallOnCompleted)
  (Widget|RemovefromParent (stale EventCreated _widget_instance)))

(event Custom|dialog%20junge
  (bind _dialogueuiinstance (CallFunction|CreateDialogueInstance 1))
  (Default|AddData _dialogueuiinstance 0 "Nach dem was so in letzter Zeit passiert ist, haben Mama und Papa sich doch wieder gut verstanden. Deswegen gingen sie zu ihrem Hochzeitstag in ein Restaurant." 18.0)
  (Default|AddData _dialogueuiinstance 0 "Ich sollte auf meine Schwester aufpassen weil sie keinen Babysitter gefunden haben. " 12.0)
  (Default|AddData _dialogueuiinstance 0 "Ich musste kurz aufs Klo gehen und hab sie im Kinderzimmer alleine gelassen." 12.0)
  (Default|AddData _dialogueuiinstance 0 "Während ich im Bad war hat sie eine Katze auf dem Balkon gesehen und wollte mit ihr spielen" 12.0)
  (Default|AddData _dialogueuiinstance 0 "Ich kam grad aus dem Bad als ich sie sah..." 8.0)
  (Default|Start _dialogueuiinstance))

(event EventCreated
  (CallFunction|HideQuestGoal)
  (Utilities|GetPaperbyName "Blatt6" true
    (:success
      _)
    (:notfound
      _))
  (Utilities|GetPaperbyName "Blatt7" true
    (:success
      _)
    (:notfound
      _))
  (Utilities|GetPaperbyName "Blatt8" true
    (:success
      _)
    (:notfound
      _))
  (Utilities|GetPaperbyName "Blatt9" true
    (:success
      _)
    (:notfound
      _))
  (Utilities|GetPaperbyName "Blatt10" true
    (:success
      _)
    (:notfound
      _))
  (bind _newsequence (Default|CreateLevelSequencePlayer (Variables|Default|GetGameMode) "/Game/Animations/Cutscenes/seq_ending2.seq_ending2"))
  (Audio|Components|Audio|Play _newsequence)
  (bind _widget_instance (Default|CreateWidget (Variables|Default|GetGameMode) "/Game/Blueprints/UI/Ending2.Ending2_C"))
  (UserInterface|Viewport|AddtoViewport _widget_instance 0)
  (Utilities|Time|SetTimerbyEvent (delegate Custom|CutsceneFinished) (Class|LevelSequencePlayer|GetLength _newsequence)))