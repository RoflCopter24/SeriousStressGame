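; Character Blueprint that offers up to two interaction choices, left and right, through an InteractionUI widget component.
; BeginPlay caches the widget and binds its left and right click events, while OnLeftChoiceChosen and OnRightChoiceChosen fire the matching interaction dispatchers.
; Tick shows the widget with the configured options and texts while the character is aimed at with a visible mesh, otherwise hiding it.
; CharacterState changes are compared but trigger nothing.
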(event EventBeginPlay
  (bind _asinteraction_ui (Utilities|Casting|CastToInteractionUI (UserInterface|GetUserWidgetObject (Variables|Default|GetInteractionWidget)))
    (:then
      (bind _output_get (Variables|Default|SetInteractionUiInstance _asinteraction_ui))
      (EventDispatchers|BindEventtoOnOptionLeftClicked _output_get (EventDispatchers|CreateEvent :!event OnLeftChoiceChosen))
      (EventDispatchers|BindEventtoOnOptionRightClicked _output_get (EventDispatchers|CreateEvent :!event OnRightChoiceChosen)))
    (:CastFailed
      (Development|PrintString "Cast failed"))))

(event Collision|EventActorBeginOverlap
  (params (OtherActor :type Actor%20Object%20Reference)))

(event EventTick
  (params (DeltaSeconds :type Float%20%28single-precision%29))
  (bind _interactionwidget (Variables|Default|GetInteractionWidget))
  (bind _bvisible (Variables|/Script/Engine.SceneComponent|GetbVisible _interactionwidget))
  ;[1 1 1] UI Stuff
  (if (and (Variables|Default|GetAimedAt) (Rendering|IsVisible (Variables|Character|GetMesh)))
    (if (not _bvisible)
      (CallFunction|ShowInteractionUI)
      (if (Utilities|Enum|NotEqual(Enum) (Variables|Default|GetCharacterState) (Variables|Default|GetLastCharState)) :!label _label
        _
        (else
          _))
      (Variables|Default|SetLastCharState (Variables|Default|GetCharacterState)))
    (elif _bvisible
      (CallFunction|HideInteractionUI)
      (goto _label))))

(fn ConstructionScript)

(fn OnLeftChoiceChosen
  (Default|CallOnLeftChoiceInteraction))

(fn OnRightChoiceChosen
  (Default|CallOnRightChoiceInteraction))

(fn ShowInteractionUI
  (bind _interactionwidget (Variables|Default|GetInteractionWidget))
  (bind _returnvalue (UserInterface|GetUserWidgetObject _interactionwidget))
  (Rendering|SetVisibility _interactionwidget true false)
  (Widget|SetVisibility _returnvalue "Visible")
  (bind _asinteraction_ui (Utilities|Casting|CastToInteractionUI _returnvalue))
  (if (Variables|Default|GetbLeftInteraction)
    (Default|EnableOptionLeft _asinteraction_ui))
  (if (Variables|Default|GetbRightInteraction)
    (Default|EnableOptionRight _asinteraction_ui))
  (Default|SetTextLeftOption _asinteraction_ui (Variables|Default|GettextLeftInteraction))
  (Default|SetTextRightOption _asinteraction_ui (Variables|Default|GettextRightInteraction)))

(fn HideInteractionUI
  (bind _interactionwidget (Variables|Default|GetInteractionWidget))
  (Rendering|SetVisibility _interactionwidget false false)
  (Widget|SetVisibility (UserInterface|GetUserWidgetObject _interactionwidget) "Hidden"))